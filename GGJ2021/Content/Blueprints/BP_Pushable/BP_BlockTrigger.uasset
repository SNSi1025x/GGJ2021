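; Puzzle trigger that opens a linked door when a BP_PushableObject overlaps it.
; On overlap it turns on the block's cube physics and ends its interact outline.
; After a short delay it disables player input, cuts to CineCamera, calls Solved on the door, then restores view and input.
; It then adjusts the first-person character's sanity and flashlight charge by success amounts, clamped to their maximums.
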(event `self.ReceiveBeginPlay`
  (`self.SetActorTickEnabled` false))

(event `self.ReceiveActorBeginOverlap`
  (params (OtherActor :type "Actor Object Reference")))

(event `self.ReceiveTick`
  (params (DeltaSeconds :type "Float (single-precision)"))
  (`|ExecutionSequence`))

(event `self.BlockTrigger.OnComponentBeginOverlap`
  (params (OverlappedComponent :type "PrimitiveComponent Object Reference") (OtherActor :type "Actor Object Reference") (OtherComp :type "PrimitiveComponent Object Reference") (OtherBodyIndex :type Integer) (bFromSweep :type Boolean) (SweepResult :type "HitResult Structure (by ref)"))
  (bind _asbp_pushable_object (cast `/Game/Blueprints/BP_Pushable/BP_PushableObject` OtherActor))
  (`PrimitiveComponent.SetSimulatePhysics` (`/Game/Blueprints/BP_Pushable/BP_PushableObject.Cube` _asbp_pushable_object) true)
  (`/Game/Blueprints/Components/InteractOutline.EndOverlap` (`/Game/Blueprints/BP_Pushable/BP_PushableObject.InteractOutline` _asbp_pushable_object))
  (`|ExecutionSequence`
    (:`then_0`
      (`KismetSystemLibrary.Delay` 1.0)
      (`self.DisableInput` (`GameplayStatics.GetPlayerCharacter` 0) (`GameplayStatics.GetPlayerController` 0))
      (`PlayerController.SetViewTargetWithBlend` (`GameplayStatics.GetPlayerController` 0) (`self.CineCamera`) 0.0 "VTBlend_Linear" 0.0 false)
      (`KismetSystemLibrary.Delay` 0.5)
      (`/Game/Blueprints/Interfaces/I_Puzzle.Solved` (`self.Door`) null)
      (`KismetSystemLibrary.Delay` (`self.CineTime`))
      (`PlayerController.SetViewTargetWithBlend` (`GameplayStatics.GetPlayerController` 0) (`Controller.K2_GetPawn` (`GameplayStatics.GetPlayerController` 0)) 0.0 "VTBlend_Linear" 0.0 false)
      (`self.EnableInput` (`GameplayStatics.GetPlayerCharacter` 0) (`GameplayStatics.GetPlayerController` 0))
      (bind _asfirst_person_character (cast `/Game/FirstPersonBP/Blueprints/FirstPersonCharacter` (`GameplayStatics.GetPlayerCharacter` 0)))
      (set `self.FPC` _asfirst_person_character)
      (`self.IncreaseDecreaseSanity` (`self.SanitySuccess`))
      (`self.IncreaseDecreaseCharge` (`self.ChargeSuccess`)))))

(fn `FindBlockActor`
  (for (_ _array_index) (`self.GetOverlappingActors` "/Game/Blueprints/BP_Pushable/BP_PushableObject.BP_PushableObject_C")
    _))

(fn `IncreaseDecreaseCharge`
  (params (Float :type "Float (double-precision)"))
  (set `/Game/FirstPersonBP/Blueprints/FirstPersonCharacter.fFlashlighCurrentCharge` (`KismetMathLibrary.FClamp` (+ (`/Game/FirstPersonBP/Blueprints/FirstPersonCharacter.fFlashlighCurrentCharge` (`self.FPC`)) Float) 0.0 (`/Game/FirstPersonBP/Blueprints/FirstPersonCharacter.fFlashlightMaxCharge` (`self.FPC`))) (`self.FPC`)))

(fn `IncreaseDecreaseSanity`
  (params (Float :type "Float (double-precision)"))
  (set `/Game/FirstPersonBP/Blueprints/FirstPersonCharacter.fCurrentSanity` (`KismetMathLibrary.FClamp` (+ (`/Game/FirstPersonBP/Blueprints/FirstPersonCharacter.fCurrentSanity` (`self.FPC`)) Float) 0.0 (`/Game/FirstPersonBP/Blueprints/FirstPersonCharacter.fMaxSanity` (`self.FPC`))) (`self.FPC`)))

(fn `UserConstructionScript`)