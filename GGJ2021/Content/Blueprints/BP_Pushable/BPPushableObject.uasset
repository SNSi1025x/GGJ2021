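; Pushable object that, on interaction, picks a grab spot for a character carrying a BP_Push_Pull component.
; Grab spots come from the PushPullTransform array, each previewed with an arrow component by the construction script.
; HandleInteraction finds the nearest spot within the component's range by squared 2D distance, then computes a world transform raised by capsule half-height.
; That result is only drawn as a debug sphere, with no movement applied; failures print a reason.
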(event `InputAction|Interact`
  (params (Key :type "Key Structure")))

(event `/Game/Blueprints/I_Interact.Interacted`
  (params (Player :type "/Game/FirstPersonBP/Blueprints/FirstPersonCharacter Object Reference"))
  (`self.HandleInteraction` Player))

(fn `FindClosestPushTransform`
  (params (CharacterLocation :type "Vector2D Structure") (fPushRange :type "Float (double-precision)"))
  (returns (iBestIndex :type Integer))
  (locals (CurrentTransformIndex :type Integer) (CurrentDistanceSq :type "Float (double-precision)" :default 0.0) (ClosestDistanceSq :type "Float (double-precision)") (ClosestTransformIndex :type Integer))
  ;[1 1 1] Finds closest transform out of array
  (for (_array_element _array_index) (`self.PushPullTransform`)
    (set `local.CurrentTransformIndex` _array_index)
    (bind _output_get (set `local.CurrentDistanceSq` (`KismetMathLibrary.DistanceSquared2D` (`KismetMathLibrary.Conv_VectorToVector2D` (`KismetMathLibrary.TransformLocation` (`self.GetTransform`) (.location _array_element))) (`local.CharacterLocation`))))
    (if (<= _output_get (`KismetMathLibrary.Square` (`local.fPushRange`)))
      (if (or (<= (`local.CurrentDistanceSq`) (`local.ClosestDistanceSq`)) (<= (`local.ClosestTransformIndex`) 0))
        (set `local.ClosestTransformIndex` (`local.CurrentTransformIndex`))
        (set `local.ClosestDistanceSq` (`local.CurrentDistanceSq`)))))
  (return (`local.ClosestTransformIndex`)))

(fn `HandleInteraction`
  (params (Character :type "Character Object Reference"))
  (locals (PushPullComponent :type "/Game/Blueprints/BP_Pushable/BP_Push_Pull Object Reference") (CharacterPreTransform :type "Transform Structure") (CharacterNewTransform :type "Transform Structure"))
  (`/Engine/EditorBlueprintResources/StandardMacros.IsValid` Character
    (:`Is Valid`
      (bind _output_get (set `local.PushPullComponent` (`self.GetComponentByClass` Character "/Game/Blueprints/BP_Pushable/BP_Push_Pull.BP_Push_Pull_C")))
      (`/Engine/EditorBlueprintResources/StandardMacros.IsValid` _output_get
        (:`Is Valid`
          (set `local.CharacterPreTransform` (`self.GetTransform` (`local.Character`)))
          (bind _ibestindex (`self.FindClosestPushTransform` (`KismetMathLibrary.Conv_VectorToVector2D` (`self.K2_GetActorLocation` (`local.Character`))) (`/Game/Blueprints/BP_Pushable/BP_Push_Pull.fPushPullRange` (`local.PushPullComponent`))))
          (if (>= _ibestindex 0)
            (bind (_returnvalue_location _returnvalue_rotation _returnvalue_scale) (`KismetMathLibrary.BreakTransform` (`KismetMathLibrary.ComposeTransforms` (`|GetArrayItem` (`self.PushPullTransform`) _ibestindex) (`self.GetTransform`))))
            (bind _output_get_2 (set `local.CharacterNewTransform` (`KismetMathLibrary.MakeTransform` (+ _returnvalue_location (`KismetMathLibrary.MakeVector` 0.0 0.0 (`CapsuleComponent.GetScaledCapsuleHalfHeight` (`Character.CapsuleComponent` (`local.Character`))))) _returnvalue_rotation _returnvalue_scale)))
            (`KismetSystemLibrary.DrawDebugSphere` (.location _output_get_2) 20.0 12 (struct :`R` 1.0 :`G` 0.26093 :`A` 1.0) 2.0 1.0)
            (else
              (`self.FailedInfo` "No Push Pull Transform Found"))))
        (:`Is Not Valid`
          (`self.FailedInfo` "Character Does Not Have Push Pull Component"))))
    (:`Is Not Valid`
      (`self.FailedInfo` "Character Not Valid"))))

(fn `UserConstructionScript`
  (for _array_element (`self.PushPullTransform`)
    (`AddComponent|NODE_AddArrowComponent-0` :`RelativeTransform` _array_element)))