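; Pushable object actor that snaps an interacting character to a preset push/pull point and starts a push.
; Construction adds an arrow per PushPullTransform; FindClosestPushTransform picks one within the component's range, though its comparison favors farther points.
; Debug-drawn capsule and line traces check room, floor slope and walls before teleporting the character and calling BeginPush on its BP_Push_Pull component.
; Failures print their reason on screen.
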(event `InputAction|Interact`
  (params (Key :type "Key Structure")))

(event `/Game/Blueprints/Interfaces/I_Interact.Interacted`
  (params (Player :type "/Game/FirstPersonBP/Blueprints/FirstPersonCharacter Object Reference"))
  (`self.HandleInteraction` Player))

(fn `FindClosestPushTransform`
  (params (CharacterLocation :type "Vector2D Structure") (fPushRange :type "Float (double-precision)"))
  (returns (iBestIndex :type Integer))
  (locals (CurrentTransformIndex :type Integer) (CurrentDistanceSq :type "Float (double-precision)" :default 0.0) (ClosestDistanceSq :type "Float (double-precision)") (ClosestTransformIndex :type Integer) (bExectuting :type Boolean))
  ;[1 1 1] Finds closest transform out of array
  (for (_array_element _array_index) (`self.PushPullTransform`)
    (set `local.CurrentTransformIndex` _array_index)
    (bind _output_get (set `local.CurrentDistanceSq` (`KismetMathLibrary.DistanceSquared2D` (`KismetMathLibrary.Conv_VectorToVector2D` (`KismetMathLibrary.TransformLocation` (`self.GetTransform`) (.location _array_element))) (`local.CharacterLocation`))))
    (if (< _output_get (`KismetMathLibrary.Square` (`local.fPushRange`)))
      (if (or (< (`local.ClosestDistanceSq`) (`local.CurrentDistanceSq`)) (< (`local.ClosestTransformIndex`) 0))
        (set `local.ClosestTransformIndex` (`local.CurrentTransformIndex`))
        (set `local.ClosestDistanceSq` (`local.CurrentDistanceSq`)))))
  (return (`local.ClosestTransformIndex`)))

(fn `HandleInteraction`
  (params (Character :type "Character Object Reference"))
  (locals (PushPullComponent :type "/Game/Blueprints/BP_Pushable/BP_Push_Pull Object Reference") (CharacterNewTransform :type "Transform Structure"))
  (bind _characternewtransform_location (`KismetMathLibrary.BreakTransform` (`local.CharacterNewTransform`)))
  (bind _characternewtransform_location_2 (`KismetMathLibrary.BreakTransform` (`local.CharacterNewTransform`)))
  (bind _capsulecomponent (`Character.CapsuleComponent` (`local.Character`)))
  (`/Engine/EditorBlueprintResources/StandardMacros.IsValid` Character
    (:`Is Valid`
      (bind _output_get (set `local.PushPullComponent` (`self.GetComponentByClass` Character "/Game/Blueprints/BP_Pushable/BP_Push_Pull.BP_Push_Pull_C")))
      (`/Engine/EditorBlueprintResources/StandardMacros.IsValid` _output_get
        (:`Is Valid`
          (bind _ibestindex (`self.FindClosestPushTransform` (`KismetMathLibrary.Conv_VectorToVector2D` (`self.K2_GetActorLocation` (`local.Character`))) (`/Game/Blueprints/BP_Pushable/BP_Push_Pull.fPushPullRange` (`local.PushPullComponent`))))
          (if (>= _ibestindex 0)
            (bind (_returnvalue_location _returnvalue_rotation _returnvalue_scale) (`KismetMathLibrary.BreakTransform` (`KismetMathLibrary.ComposeTransforms` (`|GetArrayItem` (`self.PushPullTransform`) _ibestindex) (`self.GetTransform`))))
            (bind _output_get_2 (set `local.CharacterNewTransform` (`KismetMathLibrary.MakeTransform` (+ _returnvalue_location (`KismetMathLibrary.MakeVector` 0.0 0.0 (- (`CapsuleComponent.GetScaledCapsuleHalfHeight` (`Character.CapsuleComponent` (`local.Character`))) 2.0))) _returnvalue_rotation _returnvalue_scale)))
            (`KismetSystemLibrary.DrawDebugSphere` (.location _output_get_2) 20.0 12 (struct :`R` 1.0 :`G` 0.26093 :`A` 1.0) 2.0 1.0)
            (bind _outhit (`KismetSystemLibrary.CapsuleTraceSingle` :`Start` (+ _characternewtransform_location_2 (0.0 0.0 70.0)) :`End` (- _characternewtransform_location_2 (0.0 0.0 100.0)) :`Radius` (`CapsuleComponent.GetScaledCapsuleRadius` _capsulecomponent) :`HalfHeight` (`CapsuleComponent.GetScaledCapsuleHalfHeight` _capsulecomponent) :`TraceChannel` "TraceTypeQuery1" :`DrawDebugType` "ForDuration" :`DrawTime` 2.0))
            (bind (_bblockinghit _binitialoverlap _time _distance _location _impactpoint _normal _impactnormal) (`GameplayStatics.BreakHitResult` _outhit))
            (if (not _binitialoverlap)
              (if (< (`CharacterMovementComponent.K2_GetWalkableFloorZ` (`Character.CharacterMovement` (`local.Character`))) (.z _impactnormal))
                (bind (_outhit_2 _returnvalue) (`KismetSystemLibrary.LineTraceSingle` (`self.K2_GetActorLocation`) _characternewtransform_location "TraceTypeQuery1" false (`|MakeArray` (`local.Character`) :!type "Actor Object Reference") "ForDuration" true (struct :`R` 1.0 :`A` 1.0) (struct :`G` 1.0 :`A` 1.0) 2.0))
                (if (not _returnvalue)
                  (`self.K2_SetActorTransform` (`local.Character`) (`local.CharacterNewTransform`) false true)
                  (`/Game/Blueprints/BP_Pushable/BP_Push_Pull.BeginPush` (`local.PushPullComponent`) self)
                  (else
                    (`self.FailedInfo` "Wall in way")))
                (else
                  (`self.FailedInfo` "Floor too steep")))
              (else
                (`self.FailedInfo` "No room")))
            (else
              (`self.FailedInfo` "No Push Pull Transform Found"))))
        (:`Is Not Valid`
          (`self.FailedInfo` "Character Does Not Have Push Pull Component"))))
    (:`Is Not Valid`
      (`self.FailedInfo` "Character Not Valid"))))

(fn `UserConstructionScript`
  (for _array_element (`self.PushPullTransform`)
    (`AddComponent|NODE_AddArrowComponent-0` :`RelativeTransform` _array_element)))