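; Actor component that lets its owning Character push a pushable actor, with release not yet implemented (EndPush is empty).
; BeginPush attaches the Character to the pushable, constrains movement to the plane normal to its right vector, disables orient-to-movement and enables tick.
; Tick sweeps the pushable along the owner's forward vector at FPushPullSpeed, carrying the attached Character, and prints collision debug text.
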(event `self.ReceiveBeginPlay`
  (`self.SetComponentTickEnabled` false))

(event `self.ReceiveTick`
  (params (DeltaSeconds :type "Float (single-precision)"))
  (bind _currentpushable (`self.CurrentPushable`)
    (:`then`
      (bind _sweephitresult (`Actor.K2_AddActorWorldOffset` _currentpushable (* (`Actor.GetActorForwardVector` (`self.GetOwner`)) (* DeltaSeconds (`self.fPushPullSpeed`))) true false))
      (bind (_bblockinghit _binitialoverlap _time _distance _location _impactpoint _normal _impactnormal _physmat _hitactor) (`GameplayStatics.BreakHitResult` _sweephitresult))
      (`KismetSystemLibrary.PrintString` (`KismetStringLibrary.Concat_StrStr` "Collided with: " (`KismetSystemLibrary.GetDisplayName` _hitactor)) true true (select `bool` _bblockinghit :`false` (struct :`R` 1.0 :`G` 0.904667 :`A` 1.0) :`true` (struct :`R` 1.0 :`A` 1.0) :!type "LinearColor Structure")))
    (:`else`)))

(fn `BeginPush`
  (params (Pushable :type "/Game/Blueprints/BP_Pushable/Old_MayComeBackTo_BPPushableObject Object Reference"))
  (locals (OwningCharacter :type "Character Object Reference"))
  (bind _owningcharacter (`local.OwningCharacter`))
  (bind _charactermovement (`Character.CharacterMovement` _owningcharacter))
  (if (not (`KismetSystemLibrary.IsValid` (`self.CurrentPushable`)))
    (bind _ascharacter (cast `Character` (`self.GetOwner`)))
    (set `local.OwningCharacter` _ascharacter)
    (bind _output_get (set `self.CurrentPushable` (`local.Pushable`)))
    (`Actor.K2_AttachToActor` (`local.OwningCharacter`) _output_get "None" "KeepWorld" "KeepWorld" "KeepWorld" true)
    (`MovementComponent.SetPlaneConstraintEnabled` _charactermovement true)
    (`MovementComponent.SetPlaneConstraintNormal` _charactermovement (`Actor.GetActorRightVector` _owningcharacter))
    (set `CharacterMovementComponent.bOrientRotationToMovement` false _charactermovement)
    (`self.SetComponentTickEnabled` true)))

(fn `EndPush`)