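; Hint system actor that controls a hint light and flags when a hint is available based on the player's sanity.
; ToggleLight fades the light's intensity and color temperature in or out through timelines, updating LightOn and visibility, which BeginPlay initializes.
; Tick sets HintReady when the cooldown is ready and, after a short delay, FirstPersonCharacter sanity is at or below a threshold.
; An older sanity-driven automatic fade remains disconnected.
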(event `self.ReceiveBeginPlay`
  (bind _lightcomponent (`Light.LightComponent` (`self.HintLight`)))
  ;[1 1 1] Check if light is on and set its visibility
  (if (`self.LightOn`)
    (`SceneComponent.SetVisibility` _lightcomponent true false)
    (else
      (`SceneComponent.SetVisibility` _lightcomponent false false))))

(event `ToggleLight`
  (bind _lighton (`self.LightOn`))
  (bind _lightcomponent (`Light.LightComponent` (`self.HintLight`)))
  ;[1 1 1] Toggles light
  (if (not _lighton)
    (bind (_direction _foutput _fcolortemperature) (`Timeline|ToggleFadeOn` :!via `PlayFromStart`)
      (:`Update`
        (`SceneComponent.SetVisibility` _lightcomponent true false)
        (`LightComponent.SetIntensity` _lightcomponent _foutput)
        (`LightComponent.SetTemperature` _lightcomponent _fcolortemperature)
        (set `self.LightOn` true)))
    (elif _lighton
      (bind (_direction_2 _foutput_2 _fcolortemp) (`Timeline|ToggleFadeOut` :!via `PlayFromStart`)
        (:`Update`
          (`LightComponent.SetIntensity` _lightcomponent _foutput_2)
          (`LightComponent.SetTemperature` _lightcomponent _fcolortemp)
          (set `self.LightOn` false))
        (:`Finished`
          (`SceneComponent.SetVisibility` _lightcomponent false false))))))

(event `self.ReceiveTick`
  (params (DeltaSeconds :type "Float (single-precision)"))
  (`|ExecutionSequence`
    (:`then_1`
      ;[1 1 1] Determine if menu can be opened
      (if (`self.bHintCooldownReady`)
        (`KismetSystemLibrary.Delay` 0.15)
        (bind _asfirst_person_character (cast `/Game/FirstPersonBP/Blueprints/FirstPersonCharacter` (`GameplayStatics.GetPlayerCharacter` 0)))
        (set `self.HintReady` (<= (`/Game/FirstPersonBP/Blueprints/FirstPersonCharacter.fCurrentSanity` _asfirst_person_character) (`self.fSanityThreshold`)))
        (else
          (set `self.HintReady` false))))))

(fn `UserConstructionScript`)