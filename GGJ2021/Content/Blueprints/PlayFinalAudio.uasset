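; Trigger actor that plays a two-part audio sequence, apparently the final audio going by its name, when its box is overlapped.
; The overlap handler destroys the box so it cannot retrigger, without filtering which actor entered.
; It adds audio components to the player character and plays them in turn, separated by a fixed delay.
; After a last delay, the actor destroys itself.
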(event `self.Box.OnComponentBeginOverlap`
  (params (OverlappedComponent :type "PrimitiveComponent Object Reference") (OtherActor :type "Actor Object Reference") (OtherComp :type "PrimitiveComponent Object Reference") (OtherBodyIndex :type Integer) (bFromSweep :type Boolean) (SweepResult :type "HitResult Structure (by ref)"))
  (`ActorComponent.K2_DestroyComponent` (`self.Box`))
  (bind _returnvalue (`AddComponent|NODE_AddAudioComponent-0` :`self` (`GameplayStatics.GetPlayerCharacter` 0)))
  (`AudioComponent.Play` _returnvalue 0.0)
  (`KismetSystemLibrary.Delay` 5.0)
  (bind _returnvalue_2 (`AddComponent|NODE_AddAudioComponent-2` :`self` (`GameplayStatics.GetPlayerCharacter` 0)))
  (`AudioComponent.Play` _returnvalue_2 0.0)
  (`KismetSystemLibrary.Delay` 4.0)
  (`self.K2_DestroyActor`))

(fn `UserConstructionScript`)