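; Door actor that swings its mesh open or closed when the player interacts, or in response to puzzle and lever events.
; A trigger box enables input and opens a gate for the first-person character, letting Interact toggle the door unless locked.
; Solved acts only when IsClosed is true, LeverToggle only when false, and both bypass the lock.
; DoorAnimation flips IsClosed and plays or reverses a timeline that lerps the door's yaw.
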(event `/Game/Blueprints/Interfaces/I_BlockPuzzle.Solved`
  (params (Block :type "/Game/Blueprints/BP_Pushable/BP_PushableObject Object Reference"))
  (if (`self.isClosed`)
    (if (== (`self.isClosed`) true) :!label _label
      (set `self.isClosed` false)
      (bind (_direction _door) (`Timeline|Door Timeline` :!via `ReverseFromEnd` :!label _label_2)
        (:`Update`
          (`SceneComponent.K2_SetRelativeRotation` (`self.InteriorDoor_InteriorDoor`) (`KismetMathLibrary.MakeRotator` 0.0 0.0 (`KismetMathLibrary.Lerp` (`self.DoorOpenAngle`) (`self.DoorCloseAngle`) _door)) false false)
          (`KismetSystemLibrary.PrintString` (`KismetStringLibrary.Concat_StrStr` "Door is closed: " (`KismetStringLibrary.Conv_BoolToString` (`self.isClosed`))) true true (struct :`G` 0.66 :`B` 1.0 :`A` 1.0) 0.0)))
      (else
        (set `self.isClosed` true)
        (goto _label_2 :!via `PlayFromStart`)))))

(event `self.ReceiveTick`
  (params (DeltaSeconds :type "Float (single-precision)")))

(event `/Game/Blueprints/Interfaces/I_Lever.LeverToggle`
  (params (Lever :type "/Game/Blueprints/PuzzleBPs/BPLever Object Reference"))
  (if (not (`self.isClosed`))
    (goto _label)))

(event `InputAction|Interact`
  (params (Key :type "Key Structure"))
  (:`Pressed`
    (if (not (`self.isLocked`))
      (`/Engine/EditorBlueprintResources/StandardMacros.Gate` true :!label _label_3
        (:`Exit`
          (goto _label))))))

(event `self.Box.OnComponentBeginOverlap`
  (params (OverlappedComponent :type "PrimitiveComponent Object Reference") (OtherActor :type "Actor Object Reference") (OtherComp :type "PrimitiveComponent Object Reference") (OtherBodyIndex :type Integer) (bFromSweep :type Boolean) (SweepResult :type "HitResult Structure (by ref)"))
  (cast `/Game/FirstPersonBP/Blueprints/FirstPersonCharacter` OtherActor)
  (`self.EnableInput` (`GameplayStatics.GetPlayerController` 0))
  (goto _label_3 :!via `Open`))

(event `self.Box.OnComponentEndOverlap`
  (params (OverlappedComponent :type "PrimitiveComponent Object Reference") (OtherActor :type "Actor Object Reference") (OtherComp :type "PrimitiveComponent Object Reference") (OtherBodyIndex :type Integer))
  (cast `/Game/FirstPersonBP/Blueprints/FirstPersonCharacter` OtherActor)
  (`self.DisableInput` (`GameplayStatics.GetPlayerController` 0))
  (goto _label_3 :!via `Close`))

(fn `UserConstructionScript`)