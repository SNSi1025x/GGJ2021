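; Tarot card pickup actor that the first-person player can interact with when nearby.
; Entering the sphere while the mesh was recently rendered shows a widget prompt, enables input and opens a gate; leaving reverses all three.
; Pressing Interact through the open gate plays the pickup sound at the mesh and hands off to MouseChangeScene's Interact.
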(event `self.ReceiveBeginPlay`
  (`self.SetInteractVisibility` false))

(event `InputAction|Interact`
  (params (Key :type "Key Structure"))
  (:`Pressed`
    (`/Engine/EditorBlueprintResources/StandardMacros.Gate` true :!label _label
      (:`Exit`
        (`self.PlaySound` "/Game/Sound/SoundCues/SFX/TarotCard/CUE_TarotCardPickup.CUE_TarotCardPickup")
        (`/Game/Blueprints/Components/MouseChangeScene.Interact` (`self.MouseChangeScene`))))))

(event `self.Sphere.OnComponentBeginOverlap`
  (params (OverlappedComponent :type "PrimitiveComponent Object Reference") (OtherActor :type "Actor Object Reference") (OtherComp :type "PrimitiveComponent Object Reference") (OtherBodyIndex :type Integer) (bFromSweep :type Boolean) (SweepResult :type "HitResult Structure (by ref)"))
  (bind _asfirst_person_character (cast `/Game/FirstPersonBP/Blueprints/FirstPersonCharacter` OtherActor))
  (set `self.FPC` _asfirst_person_character)
  (if (`PrimitiveComponent.WasRecentlyRendered` (`self.StaticMeshComponent`) 0.2)
    (`self.SetInteractText` "Press 'E' to pickup!")
    (`self.SetInteractVisibility` true)
    (`self.EnableInput` (`GameplayStatics.GetPlayerController` 0))
    (goto _label :!via `Open`)))

(event `self.Sphere.OnComponentEndOverlap`
  (params (OverlappedComponent :type "PrimitiveComponent Object Reference") (OtherActor :type "Actor Object Reference") (OtherComp :type "PrimitiveComponent Object Reference") (OtherBodyIndex :type Integer))
  (cast `/Game/FirstPersonBP/Blueprints/FirstPersonCharacter` OtherActor)
  (`self.SetInteractVisibility` false)
  (`self.DisableInput` (`GameplayStatics.GetPlayerController` 0))
  (goto _label :!via `Close`))

(fn `ComponentsToSave`
  (returns (Components :type "Array of ActorComponent Object Reference"))
  (return))

(fn `PlaySound`
  (params (Sound :type "SoundBase Object Reference"))
  (`GameplayStatics.SpawnSoundAtLocation` Sound (`SceneComponent.K2_GetComponentLocation` (`self.StaticMeshComponent`)) (struct) 1.0 1.0 0.0 null null))

(fn `SetInteractText`
  (params (InText :type Text))
  (bind _asinteract (cast `/Game/Items/Interact` (`WidgetComponent.GetWidget` (`self.Interact`))))
  (bind _interacttext (`/Game/Items/Interact.InteractText` _asinteract))
  (`TextBlock.SetText` _interacttext InText)
  (`TextBlock.SetFont` _interacttext (`self.Font`)))

(fn `SetInteractVisibility`
  (params (bNewVisibility :type Boolean))
  (`SceneComponent.SetVisibility` (`self.Interact`) bNewVisibility false))

(fn `UserConstructionScript`)