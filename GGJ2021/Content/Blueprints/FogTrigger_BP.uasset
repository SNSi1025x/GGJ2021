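; FogTrigger_BP is a trigger actor that fades a referenced fog actor's start distance as the first-person character enters or leaves it.
; Begin overlap plays one timeline to lerp the start distance from FogON to FogOFF through its FogHide track.
; End overlap runs a second timeline in reverse from its end, driving the same lerp to bring the fog back.
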(event `self.ReceiveActorBeginOverlap`
  (params (OtherActor :type "Actor Object Reference"))
  (cast `/Game/FirstPersonBP/Blueprints/FirstPersonCharacter` OtherActor)
  (bind (_direction _fog_hide) (`Timeline|Timeline_0`)
    (:`Update`
      (`ExponentialHeightFogComponent.SetStartDistance` (`ExponentialHeightFog.Component` (`self.Fog`)) (`KismetMathLibrary.Lerp` (`self.Fog ON`) (`self.Fog OFF`) _fog_hide)))))

(event `self.ReceiveActorEndOverlap`
  (params (OtherActor :type "Actor Object Reference"))
  (cast `/Game/FirstPersonBP/Blueprints/FirstPersonCharacter` OtherActor)
  (bind (_direction _fog_hide) (`Timeline|Timeline_1` :!via `ReverseFromEnd`)
    (:`Update`
      (`ExponentialHeightFogComponent.SetStartDistance` (`ExponentialHeightFog.Component` (`self.Fog`)) (`KismetMathLibrary.Lerp` (`self.Fog ON`) (`self.Fog OFF`) _fog_hide)))))

(fn `UserConstructionScript`)