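; A light actor that switches itself off once a linked trigger object becomes hidden.
; Tick polls ObjTrigger's hidden state until it is set, then zeroes the point light intensity and destroys the LightDetector and SanityFlashlightTrigger actors.
; An IsOut flag makes the shutdown happen only once.
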(event `self.ReceiveTick`
  (params (DeltaSeconds :type "Float (single-precision)"))
  (if (`self.IsOut`)
    _
    (elif (`Actor.bHidden` (`self.ObjTrigger`))
      (`LightComponent.SetIntensity` (`self.PointLightComponent`) 0.0)
      (`self.K2_DestroyActor` (`self.LightDetector`))
      (`self.K2_DestroyActor` (`self.SanityFlashlightTrigger`))
      (set `self.IsOut` true))))

(fn `UserConstructionScript`)