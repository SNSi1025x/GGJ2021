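; DialogueHolder feeds dialogue lines from its Dialogues array to a DialogueSystem widget it creates at BeginPlay.
; AddDialogue takes line indices, retrying every second while IsInPlay marks another sequence as running.
; Lines are formatted as "Character:Line" text and passed to the widget's PlayQueue.
; Requests over two lines loop through timed, speaker-checked batches using a countdown; shorter ones match indices by scanning Dialogues.
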(event `self.ReceiveBeginPlay`
  (bind _returnvalue (`|CreateWidget` "/Game/Blueprints/Widgets/DialogueSystem.DialogueSystem_C"))
  (`UserWidget.AddToViewport` _returnvalue 0)
  (set `self.DialogueReference` _returnvalue))

(event `AddDialogue`
  (params (IndexToPlay :type "Array of Integer"))
  (bind _returnvalue (`KismetArrayLibrary.Array_Length` IndexToPlay))
  (bind _dialoguetosend (`self.DialogueToSend`))
  (bind _dialoguetosend_2 (`self.DialogueToSend`))
  (bind _stringtotext (`self.StringToText`))
  (bind _stringtotext_2 (`self.StringToText`))
  (bind (_character _line) (break `/Game/Blueprints/Dialogue_System/Dialogue_Structure` (`|GetArrayItem` _dialoguetosend_2)))
  (if (`self.IsInPlay`) :!label _label
    (`KismetSystemLibrary.Delay` 1.0)
    (goto _label)
    (else
      (set `self.IndexArray` IndexToPlay)
      (`KismetArrayLibrary.Array_Clear` (`self.StringToText`))
      (if (> _returnvalue 2)
        (set `self.IsInPlay` true)
        (bind _output_get (set `self.OriginalSize` _returnvalue))
        (set `self.DecrementedSize` _output_get)
        (set `self.PreviousCharacter` "None")
        (`KismetArrayLibrary.Array_Add` _dialoguetosend_2 (`|GetArrayItem` (`self.Dialogues`) (`|GetArrayItem` (`self.IndexArray`) (- (`self.OriginalSize`) (`self.DecrementedSize`)))) :!label _label_2)
        (bind _result (`/Engine/EditorBlueprintResources/StandardMacros.DecrementInt` (`self.DecrementedSize`))
          (:`  `
            (bind _output_get_2 (set `self.CurrentCharacter` _character))
            (if (<= _result 0)
              (`KismetArrayLibrary.Array_Add` _stringtotext_2 (`KismetTextLibrary.Conv_StringToText` (`KismetStringLibrary.Concat_StrStr` _character ": " _line)))
              (`/Game/Blueprints/Widgets/DialogueSystem.Play Queue` (`self.DialogueReference`) _stringtotext_2)
              (`KismetSystemLibrary.Delay` 4.5)
              (`KismetArrayLibrary.Array_Clear` (`self.DialogueToSend`))
              (`KismetArrayLibrary.Array_Clear` (`self.StringToText`))
              (set `self.IsInPlay` false)
              (elif (`KismetStringLibrary.EqualEqual_StrStr` _output_get_2 (`self.PreviousCharacter`))
                (`KismetSystemLibrary.Delay` 5.0)
                (goto _label_2)
                (else
                  (`KismetArrayLibrary.Array_Add` _dialoguetosend (`|GetArrayItem` (`self.Dialogues`) (`|GetArrayItem` (`self.IndexArray`) (- (`self.OriginalSize`) (`self.DecrementedSize`)))))
                  (for _array_element _dialoguetosend
                    (bind (_character_2 _line_2) (break `/Game/Blueprints/Dialogue_System/Dialogue_Structure` _array_element))
                    (`KismetArrayLibrary.Array_Add` _stringtotext (`KismetTextLibrary.Conv_StringToText` (`KismetStringLibrary.Concat_StrStr` _character_2 ": " _line_2)))
                    (bind _output_get_3 (set `self.CurrentCharacter` _character_2))
                    (set `self.PreviousCharacter` _output_get_3))
                  (`/Game/Blueprints/Widgets/DialogueSystem.Play Queue` (`self.DialogueReference`) _stringtotext)
                  (`KismetArrayLibrary.Array_Clear` (`self.DialogueToSend`))
                  (`KismetArrayLibrary.Array_Clear` (`self.StringToText`))
                  (bind _result_2 (`/Engine/EditorBlueprintResources/StandardMacros.DecrementInt` (`self.DecrementedSize`))
                    (:`  `
                      (if (<= _result_2 0)
                        (`KismetSystemLibrary.Delay` 4.5)
                        (set `self.IsInPlay` false)
                        (else
                          (`KismetSystemLibrary.Delay` 5.0)
                          (goto _label_2))))))))))
        (else
          (set `self.IsInPlay` true)
          (for (_array_element_2 _array_index) (`self.Dialogues`)
            (for _array_element_3 (`self.IndexArray`)
              (if (== _array_index _array_element_3)
                (bind (_character_3 _line_3) (break `/Game/Blueprints/Dialogue_System/Dialogue_Structure` _array_element_2))
                (`KismetArrayLibrary.Array_Add` (`self.StringToText`) (`KismetTextLibrary.Conv_StringToText` (`KismetStringLibrary.Concat_StrStr` _character_3 ": " _line_3)))))
            (`/Game/Blueprints/Widgets/DialogueSystem.Play Queue` (`self.DialogueReference`) (`self.StringToText`))
            (`KismetSystemLibrary.Delay` 4.5)
            (set `self.IsInPlay` false)))))))

(fn `UserConstructionScript`)