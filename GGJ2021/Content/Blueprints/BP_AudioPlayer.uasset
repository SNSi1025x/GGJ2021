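; BP_AudioPlayer is an actor that plays random sounds from a Sound array through its Audio component, with an optional InitialSound first.
; AttenuationSettings is applied to the component in both the construction script and BeginPlay.
; A valid InitialSound binds OnAudioFinished to ChangeSound, chaining random picks as each sound ends.
; Without an InitialSound, ChangeSound runs once and that binding is never made.
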(event `self.ReceiveBeginPlay`
  (bind _audio (`self.Audio`))
  (set `AudioComponent.AttenuationSettings` (`self.Attenuation Settings`) (`self.Audio`))
  (bind _initialsound (`self.InitialSound`)
    (:`then`
      (`AudioComponent.SetSound` _audio _initialsound)
      (`AudioComponent.Play` _audio 0.0)
      (add `AudioComponent.OnAudioFinished` _audio (delegate `ChangeSound`)))
    (:`else`
      (`self.ChangeSound`))))

(event `ChangeSound`
  (`AudioComponent.SetSound` (`self.Audio`) (`|GetArrayItem` (`self.Sound`) (`KismetMathLibrary.RandomIntegerInRange` 0 (- (`KismetArrayLibrary.Array_Length` (`self.Sound`)) 1))))
  (`AudioComponent.Play` (`self.Audio`) 0.0))

(fn `UserConstructionScript`
  (set `AudioComponent.AttenuationSettings` (`self.Attenuation Settings`) (`self.Audio`)))