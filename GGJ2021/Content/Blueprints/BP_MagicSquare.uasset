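; Magic square puzzle actor that the player interacts with to enter a mouse scene and, once solved, receive a code.
; A box overlap shows the prompt and gates Interact input to the MouseChangeScene component.
; eRevealPanel binds Reveal to the MagicSquare widget.
; Reveal marks the puzzle solved, adds the code to the inventory and widget help text, and swaps nine reveal panels to their plane meshes.
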(event `self.ReceiveTick`
  (params (DeltaSeconds :type "Float (single-precision)")))

(event `self.ReceiveBeginPlay`
  (`self.SetActorTickEnabled` false)
  (`self.SetInteractVisibility` false))

(event `eRevealPanel`
  (if (not (`self.Solved`))
    (bind _foundwidgets (`WidgetBlueprintLibrary.GetAllWidgetsOfClass` "/Game/Blueprints/PuzzleBPs/MagicSquare/MagicSquare.MagicSquare_C"))
    (add `/Game/Blueprints/PuzzleBPs/MagicSquare/MagicSquare.RevealPanel` (`|GetArrayItem` _foundwidgets) (delegate `Reveal`))))

(event `Reveal`
  (set `self.Solved` true)
  (`ActorComponent.Deactivate` (`self.MouseChangeScene`))
  (`|ExecutionSequence`
    (:`then_0`
      (`self.SetMouseChangeScene`))
    (:`then_1`
      (`self.SwapPanel`))))

(event `InputAction|Interact`
  (params (Key :type "Key Structure"))
  (:`Pressed`
    (`/Engine/EditorBlueprintResources/StandardMacros.Gate` true :!label _label
      (:`Exit`
        (`/Game/Blueprints/Components/MouseChangeScene.Interact` (`self.MouseChangeScene`))))))

(event `self.Box.OnComponentBeginOverlap`
  (params (OverlappedComponent :type "PrimitiveComponent Object Reference") (OtherActor :type "Actor Object Reference") (OtherComp :type "PrimitiveComponent Object Reference") (OtherBodyIndex :type Integer) (bFromSweep :type Boolean) (SweepResult :type "HitResult Structure (by ref)"))
  (bind _asfirst_person_character (cast `/Game/FirstPersonBP/Blueprints/FirstPersonCharacter` OtherActor))
  (`/Engine/EditorBlueprintResources/StandardMacros.IsValid` _asfirst_person_character
    (:`Is Valid`
      (`self.SetInteractText` "Press 'E' to interact!")
      (`self.SetInteractVisibility` true)
      (`self.EnableInput` (`GameplayStatics.GetPlayerController` 0))
      (goto _label :!via `Open`))))

(event `self.Box.OnComponentEndOverlap`
  (params (OverlappedComponent :type "PrimitiveComponent Object Reference") (OtherActor :type "Actor Object Reference") (OtherComp :type "PrimitiveComponent Object Reference") (OtherBodyIndex :type Integer))
  (bind _asfirst_person_character (cast `/Game/FirstPersonBP/Blueprints/FirstPersonCharacter` OtherActor))
  (`/Engine/EditorBlueprintResources/StandardMacros.IsValid` _asfirst_person_character
    (:`Is Valid`
      (`self.SetInteractVisibility` false)
      (`self.DisableInput` (`GameplayStatics.GetPlayerController` 0))
      (goto _label :!via `Close`))))

(fn `ComponentsToSave`
  (returns (Components :type "Array of ActorComponent Object Reference"))
  (return))

(fn `SetInteractText`
  (params (Text :type Text))
  (bind _interacttext (`/Game/Items/Interact.InteractText` (cast `/Game/Items/Interact` (`WidgetComponent.GetUserWidgetObject` (`self.Widget`)) :!pure true)))
  (`TextBlock.SetText` _interacttext Text)
  (`TextBlock.SetFont` _interacttext (`self.Font`)))

(fn `SetInteractVisibility`
  (params (Visibility :type Boolean))
  (`SceneComponent.SetVisibility` (`self.Widget`) Visibility false))

(fn `SetMouseChangeScene`
  (locals (NewPlayerHelpText :type String))
  (bind _mousechangescene (`self.MouseChangeScene`))
  (bind _returnvalue (`KismetStringLibrary.Concat_StrStr` (`/Game/Blueprints/Components/MouseChangeScene.BeforeCode` _mousechangescene) (`/Game/Blueprints/Components/MouseChangeScene.Code` _mousechangescene) (`/Game/Blueprints/Components/MouseChangeScene.AfterCode` _mousechangescene)))
  (set `/Game/Blueprints/Components/MouseChangeScene.isPuzzleFinished` true _mousechangescene)
  (set `local.NewPlayerHelpText` _returnvalue)
  (set `/Game/Blueprints/Components/MouseChangeScene.Desc` _returnvalue _mousechangescene)
  (set `/Game/Blueprints/Components/MouseChangeScene.Name` "Code" _mousechangescene)
  (set `/Game/Blueprints/Components/MouseChangeScene.InputType` 2 _mousechangescene)
  (bind _asfirst_person_character (cast `/Game/FirstPersonBP/Blueprints/FirstPersonCharacter` (`GameplayStatics.GetPlayerCharacter` 0)))
  (`/Game/Blueprints/Components/Inventory.AddItem` (`/Game/FirstPersonBP/Blueprints/FirstPersonCharacter.Inventory` _asfirst_person_character) (`self.MouseChangeScene`))
  (bind _foundwidgets (`WidgetBlueprintLibrary.GetAllWidgetsOfClass` "/Game/Blueprints/PuzzleBPs/MagicSquare/MagicSquare.MagicSquare_C"))
  (`TextBlock.SetText` (`/Game/Blueprints/PuzzleBPs/MagicSquare/MagicSquare.PlayerHelpText` (`|GetArrayItem` _foundwidgets)) (`KismetTextLibrary.Conv_StringToText` (`local.NewPlayerHelpText`))))

(fn `SwapPanel`
  (bind _revealpanel8 (`self.RevealPanel8`))
  (bind _revealpanel (`self.RevealPanel`))
  (bind _revealpanel1 (`self.RevealPanel1`))
  (bind _revealpanel2 (`self.RevealPanel2`))
  (bind _revealpanel3 (`self.RevealPanel3`))
  (bind _revealpanel4 (`self.RevealPanel4`))
  (bind _revealpanel5 (`self.RevealPanel5`))
  (bind _revealpanel6 (`self.RevealPanel6`))
  (bind _revealpanel7 (`self.RevealPanel7`))
  (set `/Game/Blueprints/PuzzleBPs/MagicSquare/RevealPanel.Mesh` (`self.Plane`) _revealpanel)
  (set `/Game/Blueprints/PuzzleBPs/MagicSquare/RevealPanel.Mesh` (`self.Plane1`) _revealpanel1)
  (set `/Game/Blueprints/PuzzleBPs/MagicSquare/RevealPanel.Mesh` (`self.Plane2`) _revealpanel2)
  (set `/Game/Blueprints/PuzzleBPs/MagicSquare/RevealPanel.Mesh` (`self.Plane3`) _revealpanel3)
  (set `/Game/Blueprints/PuzzleBPs/MagicSquare/RevealPanel.Mesh` (`self.Plane4`) _revealpanel4)
  (set `/Game/Blueprints/PuzzleBPs/MagicSquare/RevealPanel.Mesh` (`self.Plane5`) _revealpanel5)
  (set `/Game/Blueprints/PuzzleBPs/MagicSquare/RevealPanel.Mesh` (`self.Plane6`) _revealpanel6)
  (set `/Game/Blueprints/PuzzleBPs/MagicSquare/RevealPanel.Mesh` (`self.Plane7`) _revealpanel7)
  (set `/Game/Blueprints/PuzzleBPs/MagicSquare/RevealPanel.Mesh` (`self.Plane8`) _revealpanel8)
  (for _array_element (`|MakeArray` _revealpanel _revealpanel1 _revealpanel2 _revealpanel3 _revealpanel4 _revealpanel5 _revealpanel6 _revealpanel7 _revealpanel8 null)
    (`/Engine/EditorBlueprintResources/StandardMacros.IsValid` _array_element
      (:`Is Valid`
        (`/Game/Blueprints/PuzzleBPs/MagicSquare/RevealPanel.SwapComponent` _array_element)))))

(fn `UserConstructionScript`)