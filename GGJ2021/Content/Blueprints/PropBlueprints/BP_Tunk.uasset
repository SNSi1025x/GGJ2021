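; Trunk prop Blueprint that opens with an animated lid, triggered by the OpenTrunk event or the L key.
; It enables input for player controller 0 on BeginPlay so the key works.
; Opening hides the Trunk component and reveals TrunkLid1 and OpenTrunkExtra.
; The TrunkOpen timeline then drives the lid's relative location and pitch, with StartRotation supplying the yaw.
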(event `self.ReceiveBeginPlay`
  (`self.EnableInput` (`GameplayStatics.GetPlayerController` 0)))

(event `OpenTrunk`
  (`SceneComponent.SetVisibility` (`self.Trunk`) false false :!label _label)
  (`SceneComponent.SetVisibility` (`self.Trunk_Lid_1_`) true false)
  (`SceneComponent.SetVisibility` (`self.Open_Trunk_Extra`) true false)
  (bind (_direction _trunktoprotation _trunktoplocation) (`Timeline|TrunkOpen`)
    (:`Update`
      (`SceneComponent.K2_SetRelativeLocationAndRotation` (`self.Trunk_Lid_1_`) _trunktoplocation (`KismetMathLibrary.MakeRotator` 0.0 _trunktoprotation (`self.StartRotation`)) false false))))

(event `Key|L`
  (params (Key :type "Key Structure"))
  (:`Pressed`
    (goto _label)))

(fn `UserConstructionScript`)