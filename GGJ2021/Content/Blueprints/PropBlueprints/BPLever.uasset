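; A lever prop that moves a referenced actor while the first-person character stands in its trigger box.
; Box overlap plays two timelines: one pitches the lever's cylinder, the other lerps the target's transform between begin and end point actors at an adjustable play rate.
; Leaving the box reverses both timelines, returning lever and object toward their start.
; The construction script applies a configurable relative transform to the lever cylinder.
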(event `self.Box.OnComponentBeginOverlap`
  (params (OverlappedComponent :type "PrimitiveComponent Object Reference") (OtherActor :type "Actor Object Reference") (OtherComp :type "PrimitiveComponent Object Reference") (OtherBodyIndex :type Integer) (bFromSweep :type Boolean) (SweepResult :type "HitResult Structure (by ref)"))
  (cast `/Game/FirstPersonBP/Blueprints/FirstPersonCharacter` OtherActor)
  (`|ExecutionSequence`
    (:`then_0`
      (bind (_direction _lever) (`Timeline|Lever` :!label _label)
        (:`Update`
          (`SceneComponent.K2_SetRelativeRotation` (`self.Cylinder`) (`KismetMathLibrary.MakeRotator` 0.0 _lever) false false))))
    (:`then_1`
      (`TimelineComponent.SetPlayRate` (`self.Lerp 0 - 1`) (`self.PlaybackRate`))
      (bind (_direction_2 _lerp) (`Timeline|Lerp 0 - 1` :!label _label_2)
        (:`Update`
          (`self.K2_SetActorTransform` (`self.ObjectToMove`) (`KismetMathLibrary.TLerp` (`self.GetTransform` (`self.BeginPoint`)) (`self.GetTransform` (`self.EndPoint`)) _lerp) false false))))))

(event `self.Box.OnComponentEndOverlap`
  (params (OverlappedComponent :type "PrimitiveComponent Object Reference") (OtherActor :type "Actor Object Reference") (OtherComp :type "PrimitiveComponent Object Reference") (OtherBodyIndex :type Integer))
  (cast `/Game/FirstPersonBP/Blueprints/FirstPersonCharacter` OtherActor)
  (`|ExecutionSequence`
    (:`then_0`
      (goto _label :!via `Reverse`))
    (:`then_1`
      (goto _label_2 :!via `Reverse`))))

(fn `UserConstructionScript`
  (`SceneComponent.K2_SetRelativeTransform` (`self.Cylinder`) (`self.LeverTransform`) false false))