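; Event-driven Shadow People variant that stays dormant until an object is picked up, then fades into view.
; BeginPlay flags it as an event before running the parent's setup.
; Tick polls whether EventTrigger is hidden, then sets IsVisible, loops the angel idle animation and drives the AngelFade material parameter from a timeline.
; The parent's Tick runs only once IsVisible is set.
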(event `self.ReceiveBeginPlay`
  (set `self.IsEvent` true)
  (`parent.ReceiveBeginPlay`))

(event `self.ReceiveTick`
  (params (DeltaSeconds :type "Float (single-precision)"))
  (bind _skeletalmesh (`self.SkeletalMesh`))
  (if (`self.IsVisible`)
    (`parent.ReceiveTick` 0.0)
    (else
      ;[1 1 1] Spawn Shadow People when an object has been picked up
      (if (`Actor.bHidden` (`self.EventTrigger`))
        (set `self.IsVisible` true)
        (`SkeletalMeshComponent.PlayAnimation` _skeletalmesh "/Game/ImportedAssets/Angel/angel_idle_anim.angel_idle_anim" true)
        (bind (_direction _fade_value) (`Timeline|event_angel_fade_in` :!via `PlayFromStart`)
          (:`Update`
            (`MeshComponent.SetScalarParameterValueOnMaterials` _skeletalmesh "AngelFade" _fade_value)))))))

(fn `UserConstructionScript`
  (`parent.UserConstructionScript`))