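; Shadow person actor that appears in the world and costs the player sanity when spotted.
; Unless flagged as an event, it fades in after a random delay by animating a FadeOut material parameter.
; Tick uses a view dot product, visibility trace and distance check to detect being seen.
; A sighting shakes the camera, applies the sanity change, optionally queues DialogueHolder dialogue, then fades out and destroys the actor.
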(event `self.ReceiveBeginPlay`
  (`|ExecutionSequence`
    (:`then_0`
      ;[1 1 1] Shadow people slowly appear when "spawned"
      (`PrimitiveComponent.SetCollisionEnabled` (`self.Body`) "NoCollision")
      (`PrimitiveComponent.SetCollisionEnabled` (`self.Head`) "NoCollision")
      (if (not (`self.IsEvent`))
        (`KismetSystemLibrary.Delay` (`KismetMathLibrary.RandomFloatInRange` (`self.EarliestSpawnTime`) (`self.LatestSpawnTime`)))
        (set `self.IsVisible` true)
        (bind (_direction _newtrack_0) (`Timeline|FadeIn` :!via `PlayFromStart`)
          (:`Update`
            (`MeshComponent.SetScalarParameterValueOnMaterials` (`self.Body`) "FadeOut" (`KismetMathLibrary.Lerp` -0.2 2.0 _newtrack_0))
            (`MeshComponent.SetScalarParameterValueOnMaterials` (`self.Head`) "FadeOut" (`KismetMathLibrary.Lerp` -0.2 2.0 _newtrack_0))))))
    (:`then_1`
      ;[1 1 1] Get FPC
      (bind _asfirst_person_character (cast `/Game/FirstPersonBP/Blueprints/FirstPersonCharacter` (`GameplayStatics.GetPlayerCharacter` 0)))
      (bind _output_get (set `self.FPC` _asfirst_person_character))
      (`/Engine/EditorBlueprintResources/StandardMacros.IsValid` _output_get
        (:`Is Not Valid`
          (`KismetSystemLibrary.PrintString` "Player not found!"))))))

(event `self.ReceiveTick`
  (params (DeltaSeconds :type "Float (single-precision)"))
  ;[1 1 1] Check if player sees the shadow person
  (if (`self.IsVisible`)
    (if (not (`self.HasBeenSeen`))
      (bind _dotproduct (`self.IsPlayerFacing` self))
      (if (`KismetMathLibrary.InRange_FloatFloat` _dotproduct 0.98)
        (bind (_outhit _returnvalue) (`KismetSystemLibrary.LineTraceSingle` (`SceneComponent.K2_GetComponentLocation` (`self.Body`)) (`self.K2_GetActorLocation` (`GameplayStatics.GetPlayerCharacter` 0)) "TraceTypeQuery1"))
        (if (not _returnvalue)
          (bind _distance (`self.Get Distance Playerto Shadow` (`self.FPC`)))
          (if (< _distance 2500.0)
            (`PlayerCameraManager.StartMatineeCameraShake` :`self` (`PlayerController.PlayerCameraManager` (`GameplayStatics.GetPlayerController` 0)) :`ShakeClass` "/Game/Blueprints/ShadowPeople_BP/ShadowShakeCamera_BP.ShadowShakeCamera_BP_C" :`Scale` 1.5)
            (`self.DecreaseSanity` (`self.SanityLostValue`))
            (`|ExecutionSequence`
              (:`then_0`
                ;[1 1 1] Shadow Person fades away after being seen
                (set `self.HasBeenSeen` true)
                (`KismetSystemLibrary.Delay` 2.0)
                (bind (_direction _newtrack_0) (`Timeline|FadeAway` :!via `PlayFromStart`)
                  (:`Update`
                    (`MeshComponent.SetScalarParameterValueOnMaterials` (`self.Body`) "FadeOut" (`KismetMathLibrary.Lerp` 2.0 -0.2 _newtrack_0))
                    (`MeshComponent.SetScalarParameterValueOnMaterials` (`self.Head`) "FadeOut" (`KismetMathLibrary.Lerp` 2.0 -0.2 _newtrack_0)))
                  (:`Finished`
                    (`self.K2_DestroyActor`))))
              (:`then_1`
                (if (`self.hasDialogue`)
                  (bind _returnvalue_2 (`GameplayStatics.GetActorOfClass` "/Game/Blueprints/Dialogue_System/DialogueHolder.DialogueHolder_C"))
                  (`/Game/Blueprints/Dialogue_System/DialogueHolder.AddDialogue` _returnvalue_2 (`self.DialogueArrayIndex`)))))))))))

(fn `DecreaseSanity`
  (params (SanityLost :type "Float (double-precision)"))
  (bind _fpc (`self.FPC`))
  (set `/Game/FirstPersonBP/Blueprints/FirstPersonCharacter.fCurrentSanity` (`KismetMathLibrary.FClamp` (+ (`/Game/FirstPersonBP/Blueprints/FirstPersonCharacter.fCurrentSanity` _fpc) SanityLost) 0.0 (`/Game/FirstPersonBP/Blueprints/FirstPersonCharacter.fMaxSanity` _fpc)) _fpc))

(fn `Get Distance Playerto Shadow`
  (params (FPC :type "/Game/FirstPersonBP/Blueprints/FirstPersonCharacter Object Reference"))
  (returns (Distance :type "Float (double-precision)"))
  (return (`self.GetDistanceTo` FPC)))

(fn `IsPlayerFacing`
  (params (Actor :type "Actor Object Reference"))
  (returns (DotProduct :type "Float (double-precision)"))
  (bind _returnvalue (`GameplayStatics.GetPlayerCameraManager` 0))
  (return (`KismetMathLibrary.Dot_VectorVector` (`KismetMathLibrary.Normal` (- (`self.K2_GetActorLocation` Actor) (`PlayerCameraManager.GetCameraLocation` _returnvalue))) (`KismetMathLibrary.Normal` (`self.GetActorForwardVector` _returnvalue)))))

(fn `OnRep_IsVisible`)

(fn `UserConstructionScript`)