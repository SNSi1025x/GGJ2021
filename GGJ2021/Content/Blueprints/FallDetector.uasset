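; FallDetector is a trigger actor that returns the player to a set location when they enter its box, presumably after a fall.
; On box overlap by a FirstPersonCharacter, it plays the HUD fade-in animation and, after a short delay, teleports the character to the LocationToMoveTo actor's position.
; After another brief delay it zeroes the character's movement velocity and plays the fade-out animation.
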(event `self.Box.OnComponentBeginOverlap`
  (params (OverlappedComponent :type "PrimitiveComponent Object Reference") (OtherActor :type "Actor Object Reference") (OtherComp :type "PrimitiveComponent Object Reference") (OtherBodyIndex :type Integer) (bFromSweep :type Boolean) (SweepResult :type "HitResult Structure (by ref)"))
  (bind _hud (`/Game/FirstPersonBP/Blueprints/FirstPersonCharacter.HUD` (`self.FPC`)))
  (bind _asfirst_person_character (cast `/Game/FirstPersonBP/Blueprints/FirstPersonCharacter` OtherActor))
  (bind _output_get (set `self.FPC` _asfirst_person_character))
  (bind _hud_2 (`/Game/FirstPersonBP/Blueprints/FirstPersonCharacter.HUD` _output_get))
  (`UserWidget.PlayAnimation` _hud_2 (`/Game/Blueprints/Widgets/HUD.FadeIn` _hud_2) 0.0 1 "Forward" 1.0 false)
  (`KismetSystemLibrary.Delay` 0.7)
  (`self.K2_SetActorLocation` _output_get (`SceneComponent.K2_GetComponentLocation` (`Actor.RootComponent` (`self.LocationToMoveTo`))) false true)
  (`KismetSystemLibrary.Delay` 0.2)
  (set `MovementComponent.Velocity` (0.0 0.0 0.0) (`Character.CharacterMovement` (`self.FPC`)))
  (`UserWidget.PlayAnimation` _hud (`/Game/Blueprints/Widgets/HUD.FadeOut` _hud) 0.0 1 "Forward" 1.0 false))

(fn `UserConstructionScript`)