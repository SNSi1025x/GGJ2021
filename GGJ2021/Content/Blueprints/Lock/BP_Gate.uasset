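; Combination-lock gate with six child-actor BP_LockTumbler dials, optionally randomized at BeginPlay, that the player solves to remove the lock.
; The LockTrigger overlap shows an interact prompt and enables input and Tick only while the player is inside.
; A delayed Tick compares tumblers to Combination, breaking each matching digit's chain with a particle effect.
; A full match fires Solved once, launching the Cube with physics before destroying the actor.
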(event `self.ReceiveBeginPlay`
  (`self.SetActorTickEnabled` false)
  (`self.RandomizeTumblers`))

(event `self.ReceiveTick`
  (params (DeltaSeconds :type "Float (single-precision)"))
  ;[1 1 1] Check for correct combo
  (`KismetSystemLibrary.Delay` 0.5)
  (`|ExecutionSequence`
    (:`then_0`
      (bind _combomatch (`self.CheckCombination`))
      (if _combomatch
        (`/Engine/EditorBlueprintResources/StandardMacros.DoOnce` false
          (:`Completed`
            (`self.Solved` false)
            (set `self.LockState` false)
            (`KismetSystemLibrary.Delay` 1.0)))))
    (:`then_1`
      (`self.CheckTumblerNumber`))))

(event `self.Solved`
  (params (Unlock :type Boolean))
  (`|ExecutionSequence`
    (:`then_0`
      (`KismetSystemLibrary.Delay` 0.7)
      (`self.K2_DestroyActor`))
    (:`then_1`
      (`KismetSystemLibrary.Delay` 0.52)
      (`PrimitiveComponent.SetSimulatePhysics` (`self.Cube`) true)
      (`PrimitiveComponent.AddImpulse` (`self.Cube`) (250.0 300.0 600.0) "None" true))))

(event `self.LockTrigger.OnComponentBeginOverlap`
  (params (OverlappedComponent :type "PrimitiveComponent Object Reference") (OtherActor :type "Actor Object Reference") (OtherComp :type "PrimitiveComponent Object Reference") (OtherBodyIndex :type Integer) (bFromSweep :type Boolean) (SweepResult :type "HitResult Structure (by ref)"))
  (bind _asfirst_person_character (cast `/Game/FirstPersonBP/Blueprints/FirstPersonCharacter` OtherActor))
  (bind _output_get (set `self.FPC` _asfirst_person_character))
  (set `/Game/Blueprints/Widgets/HUD.PopUpText` "Press E to interact." (`/Game/FirstPersonBP/Blueprints/FirstPersonCharacter.HUD` _output_get))
  (`self.SetActorTickEnabled` true)
  (`self.EnableInput` (`GameplayStatics.GetPlayerController` 0))
  (`/Engine/EditorBlueprintResources/StandardMacros.Gate` true :!via `Open` :!label _label))

(event `self.LockTrigger.OnComponentEndOverlap`
  (params (OverlappedComponent :type "PrimitiveComponent Object Reference") (OtherActor :type "Actor Object Reference") (OtherComp :type "PrimitiveComponent Object Reference") (OtherBodyIndex :type Integer))
  (bind _asfirst_person_character (cast `/Game/FirstPersonBP/Blueprints/FirstPersonCharacter` OtherActor))
  (bind _output_get (set `self.FPC` _asfirst_person_character))
  (set `/Game/Blueprints/Widgets/HUD.PopUpText` "" (`/Game/FirstPersonBP/Blueprints/FirstPersonCharacter.HUD` _output_get))
  (`self.SetActorTickEnabled` false)
  (`self.DisableInput` (`GameplayStatics.GetPlayerController` 0))
  (goto _label :!via `Close`))

(fn `BreakChains`
  (params (Chains :type "SceneComponent Object Reference"))
  (`NiagaraFunctionLibrary.SpawnSystemAtLocation` (`self.ParticleSystem`) (`SceneComponent.K2_GetComponentLocation` Chains) (`SceneComponent.K2_GetComponentRotation` Chains) (`SceneComponent.K2_GetComponentScale` Chains))
  (`ActorComponent.K2_DestroyComponent` Chains))

(fn `CheckCombination`
  (returns (ComboMatch :type Boolean))
  (bind _tumblernumber (`self.GetTumblerNumber` (`self.BP_LockTumbler`)))
  (bind _tumblernumber_2 (`self.GetTumblerNumber` (`self.BP_LockTumbler1`)))
  (bind _tumblernumber_3 (`self.GetTumblerNumber` (`self.BP_LockTumbler2`)))
  (bind _tumblernumber_4 (`self.GetTumblerNumber` (`self.BP_LockTumbler3`)))
  (bind _tumblernumber_5 (`self.GetTumblerNumber` (`self.BP_LockTumbler4`)))
  (bind _tumblernumber_6 (`self.GetTumblerNumber` (`self.BP_LockTumbler5`)))
  (return (`KismetStringLibrary.EqualEqual_StrStr` (`self.Combination`) (`KismetStringLibrary.Concat_StrStr` (`KismetStringLibrary.Conv_IntToString` _tumblernumber) (`KismetStringLibrary.Conv_IntToString` _tumblernumber_2) (`KismetStringLibrary.Conv_IntToString` _tumblernumber_3) (`KismetStringLibrary.Conv_IntToString` _tumblernumber_4) (`KismetStringLibrary.Conv_IntToString` _tumblernumber_5) (`KismetStringLibrary.Conv_IntToString` _tumblernumber_6)))))

(fn `CheckTumblerNumber`
  (bind _cylinder7 (`self.Cylinder7`))
  (bind _cylinder (`self.Cylinder`))
  (bind _cylinder1 (`self.Cylinder1`))
  (bind _cylinder2 (`self.Cylinder2`))
  (bind _cylinder5 (`self.Cylinder5`))
  (bind _cylinder6 (`self.Cylinder6`))
  (for (_array_element _array_index) (`KismetStringLibrary.GetCharacterArrayFromString` (`self.Combination`))
    (switch `int` _array_index
      (:`0`
        (bind _tumblernumber (`self.GetTumblerNumber` (`self.BP_LockTumbler`)))
        (bind _returnvalue (`KismetStringLibrary.Conv_StringToInt` _array_element))
        (if (== _tumblernumber _returnvalue)
          (`/Engine/EditorBlueprintResources/StandardMacros.IsValid` _cylinder
            (:`Is Valid`
              (`self.BreakChains` _cylinder)))))
      (:`1`
        (bind _tumblernumber_2 (`self.GetTumblerNumber` (`self.BP_LockTumbler1`)))
        (if (== _tumblernumber_2 _returnvalue)
          (`/Engine/EditorBlueprintResources/StandardMacros.IsValid` _cylinder1
            (:`Is Valid`
              (`self.BreakChains` _cylinder1)))))
      (:`2`
        (bind _tumblernumber_3 (`self.GetTumblerNumber` (`self.BP_LockTumbler2`)))
        (if (== _tumblernumber_3 _returnvalue)
          (`/Engine/EditorBlueprintResources/StandardMacros.IsValid` _cylinder2
            (:`Is Valid`
              (`self.BreakChains` _cylinder2)))))
      (:`3`
        (bind _tumblernumber_4 (`self.GetTumblerNumber` (`self.BP_LockTumbler3`)))
        (if (== _tumblernumber_4 _returnvalue)
          (`/Engine/EditorBlueprintResources/StandardMacros.IsValid` _cylinder5
            (:`Is Valid`
              (`self.BreakChains` _cylinder5)))))
      (:`4`
        (bind _tumblernumber_5 (`self.GetTumblerNumber` (`self.BP_LockTumbler4`)))
        (if (== _tumblernumber_5 _returnvalue)
          (`/Engine/EditorBlueprintResources/StandardMacros.IsValid` _cylinder6
            (:`Is Valid`
              (`self.BreakChains` _cylinder6)))))
      (:`5`
        (bind _tumblernumber_6 (`self.GetTumblerNumber` (`self.BP_LockTumbler5`)))
        (if (== _tumblernumber_6 _returnvalue)
          (`/Engine/EditorBlueprintResources/StandardMacros.IsValid` _cylinder7
            (:`Is Valid`
              (`self.BreakChains` _cylinder7))))))))

(fn `GetTumblerNumber`
  (params (Tumbler :type "ChildActorComponent Object Reference"))
  (returns (TumblerNumber :type Integer))
  (return (`/Game/Blueprints/Lock/BP_LockTumbler.TumblerNumber` (cast `/Game/Blueprints/Lock/BP_LockTumbler` (`ChildActorComponent.ChildActor` Tumbler) :!pure true))))

(fn `RandomizeTumblers`
  (if (`self.RandomizeLock`)
    (`/Game/Blueprints/Lock/BP_LockTumbler.RandomizeTumbler` (cast `/Game/Blueprints/Lock/BP_LockTumbler` (`ChildActorComponent.ChildActor` (`self.BP_LockTumbler`)) :!pure true))
    (`/Game/Blueprints/Lock/BP_LockTumbler.RandomizeTumbler` (cast `/Game/Blueprints/Lock/BP_LockTumbler` (`ChildActorComponent.ChildActor` (`self.BP_LockTumbler1`)) :!pure true))
    (`/Game/Blueprints/Lock/BP_LockTumbler.RandomizeTumbler` (cast `/Game/Blueprints/Lock/BP_LockTumbler` (`ChildActorComponent.ChildActor` (`self.BP_LockTumbler2`)) :!pure true))
    (`/Game/Blueprints/Lock/BP_LockTumbler.RandomizeTumbler` (cast `/Game/Blueprints/Lock/BP_LockTumbler` (`ChildActorComponent.ChildActor` (`self.BP_LockTumbler3`)) :!pure true))
    (`/Game/Blueprints/Lock/BP_LockTumbler.RandomizeTumbler` (cast `/Game/Blueprints/Lock/BP_LockTumbler` (`ChildActorComponent.ChildActor` (`self.BP_LockTumbler4`)) :!pure true))
    (`/Game/Blueprints/Lock/BP_LockTumbler.RandomizeTumbler` (cast `/Game/Blueprints/Lock/BP_LockTumbler` (`ChildActorComponent.ChildActor` (`self.BP_LockTumbler5`)) :!pure true))))

(fn `UserConstructionScript`)