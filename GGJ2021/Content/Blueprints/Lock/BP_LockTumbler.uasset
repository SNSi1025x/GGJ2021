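; A single lock tumbler that rotates forward or backward on its roll axis to select a digit from 0 to 9.
; Spin events play timelines that offset the saved rotation, with DoOnce gates blocking repeat spins until each finishes.
; NumberCheck maps the truncated angle, in 36-degree steps either direction, to TumblerNumber, which is printed after each spin.
; BeginPlay optionally picks a starting angle from RandomRotations.
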(event `ShowTumblerNumber`
  ;[1 1 1] Show Tumbler Number
  (`KismetSystemLibrary.PrintString` (`KismetStringLibrary.Concat_StrStr` "Tumbler Number: " (`KismetStringLibrary.Conv_IntToString` (`self.TumblerNumber`)))))

(event `self.ReceiveBeginPlay`
  ;[1 1 1] Setup and randomize tumbler number
  (if (`self.RandomizeRotation`)
    (`self.RandomizeTumbler`)
    (`self.ShowTumblerNumber`)))

(event `SpinTumbler`
  ;[1 1 1] Spin tumbler
  (`/Engine/EditorBlueprintResources/StandardMacros.DoOnce` false :!label _label
    (:`Completed`
      (bind (_direction _alpha) (`Timeline|Tumbler` :!via `PlayFromStart`)
        (:`Update`
          (bind _returnvalue (+ (`self.TumblerRotation`) _alpha))
          (`SceneComponent.K2_SetRelativeRotation` (`self.LockTumbler`) (`KismetMathLibrary.MakeRotator` _returnvalue) false false))
        (:`Finished`
          (set `self.TumblerRotation` _returnvalue)
          (`self.NumberCheck`)
          (`self.ShowTumblerNumber`)
          (`self.SpinTumblerReset`)
          (if (>= (`self.TumblerRotation`) 360.0)
            (set `self.TumblerRotation` 0.0)))))))

(event `SpinTumblerReset`
  ;[1 1 1] Spin tumbler
  (goto _label :!via `Reset`))

(event `SpinTumblerBack`
  ;[1 1 1] Spin tumbler
  (`/Engine/EditorBlueprintResources/StandardMacros.DoOnce` false :!label _label_2
    (:`Completed`
      (bind (_direction _alpha) (`Timeline|Timeline_0` :!via `PlayFromStart`)
        (:`Update`
          (bind _returnvalue (- (`self.TumblerRotation`) _alpha))
          (`SceneComponent.K2_SetRelativeRotation` (`self.LockTumbler`) (`KismetMathLibrary.MakeRotator` _returnvalue) false false))
        (:`Finished`
          (set `self.TumblerRotation` _returnvalue)
          (`self.NumberCheck`)
          (`self.ShowTumblerNumber`)
          (`self.SpinTumblerBackReset`)
          (if (<= (`self.TumblerRotation`) -360.0)
            (set `self.TumblerRotation` 0.0)))))))

(event `SpinTumblerBackReset`
  ;[1 1 1] Spin tumbler
  (goto _label_2 :!via `Reset`))

(fn `NumberCheck`
  (switch `string` (`KismetStringLibrary.Conv_IntToString` (`KismetMathLibrary.FTrunc` (`self.TumblerRotation`)))
    (:`0`
      (set `self.TumblerNumber` 0 :!label _label))
    (:`36`
      (set `self.TumblerNumber` 1 :!label _label_2))
    (:`72`
      (set `self.TumblerNumber` 2 :!label _label_3))
    (:`108`
      (set `self.TumblerNumber` 3 :!label _label_4))
    (:`144`
      (set `self.TumblerNumber` 4 :!label _label_5))
    (:`180`
      (set `self.TumblerNumber` 5 :!label _label_6))
    (:`216`
      (set `self.TumblerNumber` 6 :!label _label_7))
    (:`252`
      (set `self.TumblerNumber` 7 :!label _label_8))
    (:`288`
      (set `self.TumblerNumber` 8 :!label _label_9))
    (:`324`
      (set `self.TumblerNumber` 9 :!label _label_10))
    (:`360`
      (set `self.TumblerNumber` 0))
    (:`-36`
      (goto _label_10))
    (:`-72`
      (goto _label_9))
    (:`-108`
      (goto _label_8))
    (:`-144`
      (goto _label_7))
    (:`-180`
      (goto _label_6))
    (:`-216`
      (goto _label_5))
    (:`-252`
      (goto _label_4))
    (:`-288`
      (goto _label_3))
    (:`-324`
      (goto _label_2))
    (:`-360`
      (goto _label))))

(fn `RandomizeTumbler`
  (bind _randomrotations (`self.RandomRotations`))
  (bind _output_get (set `self.TumblerRotation` (`|GetArrayItem` _randomrotations (`KismetMathLibrary.RandomIntegerInRange` 0 (- (`KismetArrayLibrary.Array_Length` _randomrotations) 1)))))
  (`SceneComponent.K2_SetRelativeRotation` (`self.LockTumbler`) (`KismetMathLibrary.MakeRotator` _output_get) false false)
  (`self.NumberCheck`))

(fn `UserConstructionScript`)