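; BP_LevelEnd is a level-end trigger that takes the player to the end credits.
; When a FirstPersonCharacter overlaps its Box, it plays that character's HUD FadeIn animation and waits for it to finish.
; It then removes the HUD, switches to UI-only input with the mouse cursor shown, and adds the W_CreditsMenuEnd widget to the viewport.
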(event `self.Box.OnComponentBeginOverlap`
  (params (OverlappedComponent :type "PrimitiveComponent Object Reference") (OtherActor :type "Actor Object Reference") (OtherComp :type "PrimitiveComponent Object Reference") (OtherBodyIndex :type Integer) (bFromSweep :type Boolean) (SweepResult :type "HitResult Structure (by ref)"))
  (bind _asfirst_person_character (cast `/Game/FirstPersonBP/Blueprints/FirstPersonCharacter` OtherActor))
  (bind _output_get (set `self.FPC` _asfirst_person_character))
  (bind _hud (`/Game/FirstPersonBP/Blueprints/FirstPersonCharacter.HUD` _output_get))
  (bind _fadein (`/Game/Blueprints/Widgets/HUD.FadeIn` _hud))
  (`UserWidget.PlayAnimation` _hud _fadein 0.0 1 "Forward" 1.0 false)
  (`UserWidget.BindToAnimationFinished` _hud _fadein (delegate `AddCredits`)))

(event `AddCredits`
  (bind _returnvalue (`GameplayStatics.GetPlayerController` 0))
  (`Widget.RemoveFromParent` (`/Game/FirstPersonBP/Blueprints/FirstPersonCharacter.HUD` (stale `self.Box.OnComponentBeginOverlap` _output_get)))
  (`WidgetBlueprintLibrary.SetInputMode_UIOnlyEx` _returnvalue null)
  (set `PlayerController.bShowMouseCursor` true _returnvalue)
  (bind _returnvalue_2 (`|CreateWidget` "/Game/Blueprints/Widgets/W_CreditsMenuEnd.W_CreditsMenuEnd_C"))
  (`UserWidget.AddToViewport` _returnvalue_2 0))

(fn `UserConstructionScript`)