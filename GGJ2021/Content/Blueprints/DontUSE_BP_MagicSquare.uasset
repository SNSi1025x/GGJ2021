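; Magic square actor, marked DontUSE by its name, that fills a list of mesh actors for MouseChangeScene.
; On BeginPlay it adds the owner of StaticMeshComponent and of nine Plane components to MouseChangeScene's StaticMeshActors array.
; Each entry is the component's owning actor rather than the mesh component itself.
; Overlap, Tick and the construction script do nothing.
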(event `self.ReceiveBeginPlay`
  (bind _staticmeshactors (`/Game/Blueprints/Components/MouseChangeScene.StaticMeshActors` (`self.MouseChangeScene`)))
  (`KismetArrayLibrary.Array_Add` _staticmeshactors (`ActorComponent.GetOwner` (`self.Plane`)))
  (`KismetArrayLibrary.Array_Add` _staticmeshactors (`ActorComponent.GetOwner` (`self.StaticMeshComponent`)))
  (`KismetArrayLibrary.Array_Add` _staticmeshactors (`ActorComponent.GetOwner` (`self.Plane1`)))
  (`KismetArrayLibrary.Array_Add` _staticmeshactors (`ActorComponent.GetOwner` (`self.Plane2`)))
  (`KismetArrayLibrary.Array_Add` _staticmeshactors (`ActorComponent.GetOwner` (`self.Plane3`)))
  (`KismetArrayLibrary.Array_Add` _staticmeshactors (`ActorComponent.GetOwner` (`self.Plane4`)))
  (`KismetArrayLibrary.Array_Add` _staticmeshactors (`ActorComponent.GetOwner` (`self.Plane5`)))
  (`KismetArrayLibrary.Array_Add` _staticmeshactors (`ActorComponent.GetOwner` (`self.Plane6`)))
  (`KismetArrayLibrary.Array_Add` _staticmeshactors (`ActorComponent.GetOwner` (`self.Plane7`)))
  (`KismetArrayLibrary.Array_Add` _staticmeshactors (`ActorComponent.GetOwner` (`self.Plane8`))))

(fn `UserConstructionScript`)