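; Padlock actor that locks a fence gate until the player has its key, then swings it open.
; Trigger overlap shows an outline and HUD prompt, and enables Interact input through a gate only when locked with the key held, as set by PlayerHasKey.
; Interacting marks the key used, optionally adds DialogueHolder dialogue, hides the chains, and plays a timeline in reverse to move and rotate the door.
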(event `self.Unlock`)

(event `self.ReceiveBeginPlay`)

(event `InputAction|Interact`
  (params (Key :type "Key Structure"))
  (bind _chains_fence_key (`self.Chains_Fence_Key`))
  (:`Pressed`
    (if (`self.IsLocked`)
      (`/Engine/EditorBlueprintResources/StandardMacros.Gate` true :!label _label
        (:`Exit`
          (if (`self.HasKey`)
            ;[1 1 1] Unlock Padlock
            (set `self.KeyUsed` true)
            (if (`self.HasKeyDialogue`)
              (bind _returnvalue (`GameplayStatics.GetActorOfClass` "/Game/Blueprints/Dialogue_System/DialogueHolder.DialogueHolder_C"))
              (`/Game/Blueprints/Dialogue_System/DialogueHolder.AddDialogue` _returnvalue (`self.Dialogue - Unlock`)))
            (`SceneComponent.SetVisibility` _chains_fence_key false false)
            (`PrimitiveComponent.SetCollisionEnabled` _chains_fence_key "NoCollision")
            (set `self.IsLocked` false)
            (bind (_direction _door) (`Timeline|Gate Animation` :!via `ReverseFromEnd`)
              (:`Update`
                (`SceneComponent.K2_SetRelativeLocationAndRotation` (`self.Fence_door`) (`KismetMathLibrary.VLerp` (`self.GateOpenLocation`) (`self.GateClosedLocation`) _door) (`KismetMathLibrary.MakeRotator` 0.0 0.0 (`KismetMathLibrary.Lerp` (`self.gateOpenAngle`) (`self.GateClosedAngle`) _door)) false false)
                (`PrimitiveComponent.SetCollisionEnabled` (`self.StaticMeshComponent`) "NoCollision")))
            (else
              ;[1 1 1] Dialogue for interacting padlock without the right key
              (if (`self.hasNoKeyDialogue`)
                (bind _returnvalue_2 (`GameplayStatics.GetActorOfClass` "/Game/Blueprints/Dialogue_System/DialogueHolder.DialogueHolder_C"))
                (`/Game/Blueprints/Dialogue_System/DialogueHolder.AddDialogue` _returnvalue_2 (`self.No key Dialogue`))))))))))

(event `self.PlayerHasKey`
  (params (PlayHasKey :type Boolean))
  (set `self.HasKey` PlayHasKey))

(event `self.InteractTrigger.OnComponentBeginOverlap`
  (params (OverlappedComponent :type "PrimitiveComponent Object Reference") (OtherActor :type "Actor Object Reference") (OtherComp :type "PrimitiveComponent Object Reference") (OtherBodyIndex :type Integer) (bFromSweep :type Boolean) (SweepResult :type "HitResult Structure (by ref)"))
  (bind _interactoutline (`self.InteractOutline`))
  (bind _hud (`/Game/FirstPersonBP/Blueprints/FirstPersonCharacter.HUD` (`self.FPC`)))
  (bind _asfirst_person_character (cast `/Game/FirstPersonBP/Blueprints/FirstPersonCharacter` OtherActor))
  (set `self.FPC` _asfirst_person_character)
  (set `/Game/Blueprints/Components/InteractOutline.StaticMesh` (`self.StaticMeshComponent`) _interactoutline)
  (`/Game/Blueprints/Components/InteractOutline.Overlap` _interactoutline)
  (if (`self.isLocked`)
    (if (`self.HasKey`)
      (set `/Game/Blueprints/Widgets/HUD.PopUpText` "Press E To Unlock" _hud)
      (`self.EnableInput` (`GameplayStatics.GetPlayerController` 0))
      (goto _label :!via `Open`)
      (else
        (set `/Game/Blueprints/Widgets/HUD.PopUpText` "Key is required" _hud)))
    (else
      (set `/Game/Blueprints/Widgets/HUD.PopUpText` "Press E to Open Gate" _hud))))

(event `self.InteractTrigger.OnComponentEndOverlap`
  (params (OverlappedComponent :type "PrimitiveComponent Object Reference") (OtherActor :type "Actor Object Reference") (OtherComp :type "PrimitiveComponent Object Reference") (OtherBodyIndex :type Integer))
  (cast `/Game/FirstPersonBP/Blueprints/FirstPersonCharacter` OtherActor)
  (`/Game/Blueprints/Components/InteractOutline.EndOverlap` (`self.InteractOutline`))
  (set `/Game/Blueprints/Widgets/HUD.PopUpText` "" (`/Game/FirstPersonBP/Blueprints/FirstPersonCharacter.HUD` (`self.FPC`)))
  (`self.DisableInput` (`GameplayStatics.GetPlayerController` 0))
  (goto _label :!via `Close`))

(fn `PlayerUsedKey`
  (returns (usedKey :type Boolean))
  (return (`self.KeyUsed`)))

(fn `UserConstructionScript`)