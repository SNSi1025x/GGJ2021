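; Key pickup that unlocks a linked UnlockObj and goes into the first-person character's inventory.
; Box overlap shows an outline and widget prompt, opening a gate for Interact input.
; Interact messages UnlockObj through I_Unlock, adds MouseChangeScene to inventory, plays sound and particles, and optionally queues one-time dialogue.
; Tick, off at start, polls UnlockObj until the key is used, then removes the item and destroys the actor.
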(event `self.ReceiveBeginPlay`
  (`self.SetActorTickEnabled` false)
  (`self.SetInteractVisibility` false))

(event `self.ReceiveTick`
  (params (DeltaSeconds :type "Float (single-precision)"))
  (bind _usedkey (message `/Game/Blueprints/Interfaces/I_Unlock.PlayerUsedKey` (`self.UnlockObj`)))
  (if _usedkey
    (bind _fpc (`self.FPC`)
      (:`then`
        (`/Game/Blueprints/Components/Inventory.RemoveItem` (`/Game/FirstPersonBP/Blueprints/FirstPersonCharacter.Inventory` _fpc) (`self.MouseChangeScene`))
        (`self.K2_DestroyActor`))
      (:`else`))))

(event `InputAction|Interact`
  (params (Key :type "Key Structure"))
  (bind _unlockobj (`self.UnlockObj`))
  (bind _mousechangescene (`self.MouseChangeScene`))
  (:`Pressed`
    (`/Engine/EditorBlueprintResources/StandardMacros.Gate` true :!label _label
      (:`Exit`
        (message `/Game/Blueprints/Interfaces/I_Unlock.PlayerHasKey` _unlockobj true)
        (if (`KismetSystemLibrary.DoesImplementInterface` _unlockobj "/Game/Blueprints/Interfaces/I_Unlock.I_Unlock_C")
          (message `/Game/Blueprints/Interfaces/I_Unlock.Unlock` (`self.UnlockObj`))
          (`self.PlaySound` "/Game/Sound/SoundCues/SFX/Keys/CUE_Keys.CUE_Keys")
          (bind _asfirst_person_character (cast `/Game/FirstPersonBP/Blueprints/FirstPersonCharacter` (`GameplayStatics.GetPlayerCharacter` 0)))
          (`/Game/Blueprints/Components/Inventory.AddItem` (`/Game/FirstPersonBP/Blueprints/FirstPersonCharacter.Inventory` _asfirst_person_character) _mousechangescene)
          (if (`self.hasDialogue`)
            (if (not (`self.DialoguePlayed`))
              (bind _returnvalue (`GameplayStatics.GetActorOfClass` "/Game/Blueprints/Dialogue_System/DialogueHolder.DialogueHolder_C"))
              (`/Game/Blueprints/Dialogue_System/DialogueHolder.AddDialogue` _returnvalue (`self.DialogueArray`))
              (set `self.DialoguePlayed` true)
              (`NiagaraFunctionLibrary.SpawnSystemAtLocation` (`self.NiagaraParticles`) (`SceneComponent.K2_GetComponentLocation` (`self.StaticMesh`)) :!label _label_2)
              (`/Game/Blueprints/Components/MouseChangeScene.Disable` _mousechangescene)
              (`self.SetActorTickEnabled` true))
            (else
              (goto _label_2)))
          (else
            (`KismetSystemLibrary.PrintString` "DOES NOT IMPLEMENT UNLOCK INTERFACE" true true (struct :`R` 1.0 :`G` 0.076411 :`A` 1.0))))))))

(event `self.Box.OnComponentBeginOverlap`
  (params (OverlappedComponent :type "PrimitiveComponent Object Reference") (OtherActor :type "Actor Object Reference") (OtherComp :type "PrimitiveComponent Object Reference") (OtherBodyIndex :type Integer) (bFromSweep :type Boolean) (SweepResult :type "HitResult Structure (by ref)"))
  (bind _interactoutline (`self.InteractOutline`))
  (bind _asfirst_person_character (cast `/Game/FirstPersonBP/Blueprints/FirstPersonCharacter` OtherActor))
  (set `self.FPC` _asfirst_person_character)
  (set `/Game/Blueprints/Components/InteractOutline.StaticMesh` (`self.StaticMesh`) _interactoutline)
  (`/Game/Blueprints/Components/InteractOutline.Overlap` _interactoutline)
  (`self.SetActorTickEnabled` true)
  (`self.SetInteractText` "Press 'E' to pickup!")
  (`self.SetInteractVisibility` true)
  (`self.EnableInput` (`GameplayStatics.GetPlayerController` 0))
  (goto _label :!via `Open`))

(event `self.Box.OnComponentEndOverlap`
  (params (OverlappedComponent :type "PrimitiveComponent Object Reference") (OtherActor :type "Actor Object Reference") (OtherComp :type "PrimitiveComponent Object Reference") (OtherBodyIndex :type Integer))
  (cast `/Game/FirstPersonBP/Blueprints/FirstPersonCharacter` OtherActor)
  (`/Game/Blueprints/Components/InteractOutline.EndOverlap` (`self.InteractOutline`))
  (`self.SetInteractVisibility` false)
  (`self.DisableInput` (`GameplayStatics.GetPlayerController` 0))
  (goto _label :!via `Close`))

(fn `ComponentsToSave`
  (returns (Components :type "Array of ActorComponent Object Reference"))
  (return))

(fn `PlayerHasKey`
  (params (PlayHasKey :type Boolean :default false))
  (return))

(fn `PlayerUsedKey`
  (returns (usedKey :type Boolean))
  (return false))

(fn `PlaySound`
  (params (Sound :type "SoundBase Object Reference"))
  (returns (Duration :type "Float (double-precision)"))
  (`GameplayStatics.SpawnSoundAtLocation` Sound (`SceneComponent.K2_GetComponentLocation` (`self.StaticMesh`)) (struct) 1.0 1.0 0.0 null null)
  (return (`SoundBase.Duration` Sound)))

(fn `SetInteractText`
  (params (Text :type Text))
  (bind _interacttext (`/Game/Items/Interact.InteractText` (cast `/Game/Items/Interact` (`WidgetComponent.GetUserWidgetObject` (`self.WidgetInteract`)) :!pure true)))
  (`TextBlock.SetText` _interacttext Text)
  (`TextBlock.SetFont` _interacttext (`self.Font`)))

(fn `SetInteractVisibility`
  (params (Visibility :type Boolean))
  (`SceneComponent.SetVisibility` (`self.WidgetInteract`) Visibility false))

(fn `UserConstructionScript`)