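; Child door Blueprint that uses a Wall component to conceal the door, as either an Invisible Door or a Disappearing Door.
; Invisible doors start locked behind the solid wall until Reveal hides it and unlocks them.
; Disappearing doors start exposed, then get walled over when the player overlaps InteractDisappear, whose transform is set in the construction script.
; Tick suppresses the interaction prompt and outline while the player is at a locked door.
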(event `self.ReceiveBeginPlay`
  (bind _wall (`self.Wall`))
  (bind _wall_2 (`self.Wall`))
  (`parent.ReceiveBeginPlay`)
  (switch `/Game/Blueprints/Enums/Enum_Door` (`self.State`)
    (:`NewEnumerator0`
      (`PrimitiveComponent.SetCollisionEnabled` _wall_2 "QueryAndPhysics")
      (`SceneComponent.SetVisibility` _wall_2 true false)
      (set `self.isLocked` true))
    (:`NewEnumerator1`
      (`PrimitiveComponent.SetCollisionEnabled` _wall "NoCollision")
      (`SceneComponent.SetVisibility` _wall false false))))

(event `self.ReceiveActorBeginOverlap`
  (params (OtherActor :type "Actor Object Reference"))
  (`parent.ReceiveActorBeginOverlap` OtherActor))

(event `self.InteractDisappear.OnComponentBeginOverlap`
  (params (OverlappedComponent :type "PrimitiveComponent Object Reference") (OtherActor :type "Actor Object Reference") (OtherComp :type "PrimitiveComponent Object Reference") (OtherBodyIndex :type Integer) (bFromSweep :type Boolean) (SweepResult :type "HitResult Structure (by ref)"))
  (bind _wall (`self.Wall`))
  ;[1 1 1] Disappears when set to disappearing door
  (switch `/Game/Blueprints/Enums/Enum_Door` (`self.State`)
    (:`NewEnumerator1`
      (cast `/Game/FirstPersonBP/Blueprints/FirstPersonCharacter` OtherActor)
      (`SceneComponent.SetVisibility` _wall true false)
      (`PrimitiveComponent.SetCollisionEnabled` _wall "QueryAndPhysics")
      (set `/Game/Blueprints/Widgets/HUD.PopUpText` "" (`/Game/FirstPersonBP/Blueprints/FirstPersonCharacter.HUD` (`self.FPC`)))
      (`ActorComponent.Deactivate` (`self.InteractOutline`)))))

(event `Reveal`
  (bind _wall (`self.Wall`))
  (switch `/Game/Blueprints/Enums/Enum_Door` (`self.State`)
    (:`NewEnumerator0`
      (`PrimitiveComponent.SetCollisionEnabled` _wall "NoCollision")
      (`SceneComponent.SetVisibility` _wall false false)
      (set `self.isLocked` false)
      (`ActorComponent.Activate` (`self.InteractOutline`) false))))

(event `self.InteractTrigger.OnComponentBeginOverlap`
  (params (OverlappedComponent :type "PrimitiveComponent Object Reference") (OtherActor :type "Actor Object Reference") (OtherComp :type "PrimitiveComponent Object Reference") (OtherBodyIndex :type Integer) (bFromSweep :type Boolean) (SweepResult :type "HitResult Structure (by ref)"))
  (cast `/Game/FirstPersonBP/Blueprints/FirstPersonCharacter` OtherActor)
  (set `self.FPCIn` true))

(event `self.InteractTrigger.OnComponentEndOverlap`
  (params (OverlappedComponent :type "PrimitiveComponent Object Reference") (OtherActor :type "Actor Object Reference") (OtherComp :type "PrimitiveComponent Object Reference") (OtherBodyIndex :type Integer))
  (cast `/Game/FirstPersonBP/Blueprints/FirstPersonCharacter` OtherActor)
  (set `self.FPCIn` false))

(event `self.ReceiveTick`
  (params (DeltaSeconds :type "Float (single-precision)"))
  (bind _fpc (`self.FPC`))
  (`parent.ReceiveTick` DeltaSeconds)
  (`KismetSystemLibrary.Delay` 0.0001)
  (if (and (`KismetSystemLibrary.IsValid` _fpc) (`self.FPCIn`) (`self.isLocked`))
    (set `/Game/Blueprints/Widgets/HUD.PopUpText` "" (`/Game/FirstPersonBP/Blueprints/FirstPersonCharacter.HUD` _fpc))
    (`/Game/Blueprints/Components/InteractOutline.EndOverlap` (`self.InteractOutline`))))

(fn `UserConstructionScript`
  (locals (InteractTransform :type "Transform Structure") (WallTransform :type "Transform Structure"))
  (`parent.UserConstructionScript`)
  (`SceneComponent.K2_SetRelativeTransform` (`self.InteractDisappear`) (`local.InteractTransform`) false false))