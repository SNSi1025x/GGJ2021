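; Lockable interior door that the player opens and closes with the Interact input.
; Overlapping InteractTrigger shows a locked/open/close HUD prompt, enables input and opens a Gate that limits interaction to that range.
; External events Unlock, Solved (unlock and open) and LeverToggle (close if open) also drive it.
; The DoorAnimation graph flips IsClosed and plays or reverses a timeline that lerps mesh yaw between open and closed angles.
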(event `/Game/Blueprints/Interfaces/I_Unlock.Unlock`
  (set `self.isLocked` false))

(event `/Game/Blueprints/Interfaces/I_Puzzle.Solved`
  (params (Block :type "/Game/Blueprints/BP_Pushable/BP_PushableObject Object Reference"))
  (if (`self.isClosed`)
    (set `self.isLocked` false)
    (if (== (`self.isClosed`) true) :!label _label
      (set `self.isClosed` false)
      (bind (_direction _door) (`Timeline|Door Timeline` :!via `ReverseFromEnd` :!label _label_2)
        (:`Update`
          (`SceneComponent.K2_SetRelativeRotation` (`self.InteriorDoor_InteriorDoor`) (`KismetMathLibrary.MakeRotator` 0.0 0.0 (`KismetMathLibrary.Lerp` (`self.DoorOpenAngle`) (`self.DoorCloseAngle`) _door)) false false)
          (`KismetSystemLibrary.PrintString` (`KismetStringLibrary.Concat_StrStr` "Door is closed: " (`KismetStringLibrary.Conv_BoolToString` (`self.isClosed`))) true true (struct :`G` 0.66 :`B` 1.0 :`A` 1.0) 0.0)))
      (else
        (set `self.isClosed` true)
        (goto _label_2 :!via `PlayFromStart`)))))

(event `self.ReceiveTick`
  (params (DeltaSeconds :type "Float (single-precision)")))

(event `/Game/Blueprints/Interfaces/I_Lever.LeverToggle`
  (params (Lever :type "/Game/Blueprints/PuzzleBPs/BP_LeverPuzzle Object Reference"))
  (if (not (`self.isClosed`))
    (goto _label)))

(event `InputAction|Interact`
  (params (Key :type "Key Structure"))
  (:`Pressed`
    (if (not (`self.isLocked`))
      (`/Engine/EditorBlueprintResources/StandardMacros.Gate` true :!label _label_3
        (:`Exit`
          (goto _label))))))

(event `self.InteractTrigger.OnComponentBeginOverlap`
  (params (OverlappedComponent :type "PrimitiveComponent Object Reference") (OtherActor :type "Actor Object Reference") (OtherComp :type "PrimitiveComponent Object Reference") (OtherBodyIndex :type Integer) (bFromSweep :type Boolean) (SweepResult :type "HitResult Structure (by ref)"))
  (bind _asfirst_person_character (cast `/Game/FirstPersonBP/Blueprints/FirstPersonCharacter` OtherActor))
  (if (`self.isLocked`)
    (bind _hud (`/Game/FirstPersonBP/Blueprints/FirstPersonCharacter.HUD` _asfirst_person_character))
    (set `/Game/Blueprints/Widgets/HUD.PopUpText` "Door is locked" _hud)
    (elif (`self.isClosed`)
      (set `/Game/Blueprints/Widgets/HUD.PopUpText` "Press E To Open" _hud)
      (else
        (set `/Game/Blueprints/Widgets/HUD.PopUpText` "Press E To Close" _hud))))
  (`self.EnableInput` (`GameplayStatics.GetPlayerController` 0))
  (goto _label_3 :!via `Open`))

(event `self.InteractTrigger.OnComponentEndOverlap`
  (params (OverlappedComponent :type "PrimitiveComponent Object Reference") (OtherActor :type "Actor Object Reference") (OtherComp :type "PrimitiveComponent Object Reference") (OtherBodyIndex :type Integer))
  (bind _asfirst_person_character (cast `/Game/FirstPersonBP/Blueprints/FirstPersonCharacter` OtherActor))
  (set `/Game/Blueprints/Widgets/HUD.PopUpText` "" (`/Game/FirstPersonBP/Blueprints/FirstPersonCharacter.HUD` _asfirst_person_character))
  (`self.DisableInput` (`GameplayStatics.GetPlayerController` 0))
  (goto _label_3 :!via `Close`))

(fn `UserConstructionScript`)