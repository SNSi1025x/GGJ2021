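; GetFPC_BP is an actor that captures a reference to the player's FirstPersonCharacter when that character first overlaps it.
; On overlap it casts the other actor, stores it through SetFPC and sets a FoundPlayer flag so later overlaps are ignored.
; GetFPC returns the cached reference for other Blueprints to read.
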(event `self.ReceiveActorBeginOverlap`
  (params (OtherActor :type "Actor Object Reference"))
  (if (not (`self.FoundPlayer`))
    (bind _asfirst_person_character (cast `/Game/FirstPersonBP/Blueprints/FirstPersonCharacter` OtherActor))
    (bind _output_get (set `self.FPC` _asfirst_person_character))
    (`self.SetFPC` _output_get)
    (set `self.FoundPlayer` true)))

(fn `GetFPC`
  (returns (FPC :type "/Game/FirstPersonBP/Blueprints/FirstPersonCharacter Object Reference"))
  (return (`self.FPC`)))

(fn `SetFPC`
  (params (FPC :type "/Game/FirstPersonBP/Blueprints/FirstPersonCharacter Object Reference"))
  (set `self.FPC` FPC)
  (return))

(fn `UserConstructionScript`)