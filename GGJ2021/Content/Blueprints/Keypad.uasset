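; Keypad puzzle actor with a widget-component UI that checks an entered code and notifies a linked Puzzle through I_Puzzle when it matches.
; BeginPlay binds the W_Keypad code-entered event; success disables the buttons, while failure flashes "Incorrect" and re-enables them after the animation.
; Both outcomes play attenuated sounds and can queue DialogueHolder lines, with failure dialogue playing only once.
; Box overlap handlers are empty; their prompt, fade and input logic is disconnected.
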(event `self.ReceiveBeginPlay`
  (bind _asw_keypad (cast `/Game/Blueprints/Widgets/W_Keypad` (`WidgetComponent.GetUserWidgetObject` (`self.Widget`))))
  (set `/Game/Blueprints/Widgets/W_Keypad.Location` (`SceneComponent.K2_GetComponentLocation` (`self.Keypad`)) _asw_keypad)
  (bind _output_get (set `self.KeypadWidget` _asw_keypad))
  (add `/Game/Blueprints/Widgets/W_Keypad.CodeEntered` _output_get (`|CreateDelegate` :!event `CheckCode`)))

(event `self.Box.OnComponentBeginOverlap`
  (params (OverlappedComponent :type "PrimitiveComponent Object Reference") (OtherActor :type "Actor Object Reference") (OtherComp :type "PrimitiveComponent Object Reference") (OtherBodyIndex :type Integer) (bFromSweep :type Boolean) (SweepResult :type "HitResult Structure (by ref)")))

(event `self.Box.OnComponentEndOverlap`
  (params (OverlappedComponent :type "PrimitiveComponent Object Reference") (OtherActor :type "Actor Object Reference") (OtherComp :type "PrimitiveComponent Object Reference") (OtherBodyIndex :type Integer)))

(event `self.Solved`
  (params (Unlock :type Boolean))
  (bind _puzzle (`self.Puzzle`))
  (if (`KismetSystemLibrary.DoesImplementInterface` _puzzle "/Game/Blueprints/Interfaces/I_Puzzle.I_Puzzle_C")
    (message `/Game/Blueprints/Interfaces/I_Puzzle.Solved` _puzzle false)))

(fn `AnimationFinished`
  (`/Game/Blueprints/Widgets/W_Keypad.EnableButtons` (`self.KeypadWidget`)))

(fn `CheckCode`
  (params (CodeEntered :type String) (KeypadUI :type "/Game/Blueprints/Widgets/W_Keypad Object Reference"))
  (bind _keypadwidget (`self.KeypadWidget`))
  (bind _incorrect (`/Game/Blueprints/Widgets/W_Keypad.Incorrect` _keypadwidget))
  (if (`KismetStringLibrary.EqualEqual_StrStr` CodeEntered (`self.Code`))
    (`self.Solved` false)
    (set `/Game/Blueprints/Widgets/W_Keypad.CurrentCode` "" (`self.KeypadWidget`))
    (`self.PlaySound` (`self.CorrectSound`))
    (set `self.isSolved` true)
    (`/Game/Blueprints/Widgets/W_Keypad.DisableButtons` (`self.KeypadWidget`))
    (if (`self.HasCompleteDialogue`)
      (bind _returnvalue (`GameplayStatics.GetActorOfClass` "/Game/Blueprints/Dialogue_System/DialogueHolder.DialogueHolder_C"))
      (`/Game/Blueprints/Dialogue_System/DialogueHolder.AddDialogue` _returnvalue (`self.DialogueArray_Complete`)))
    (else
      (`/Game/Blueprints/Widgets/W_Keypad.DisableButtons` (`self.KeypadWidget`))
      (set `/Game/Blueprints/Widgets/W_Keypad.CurrentCode` "" _keypadwidget)
      (`TextBlock.SetText` (`/Game/Blueprints/Widgets/W_Keypad.CodeText` _keypadwidget) "Incorrect")
      (`UserWidget.PlayAnimation` _keypadwidget _incorrect 0.0 2 "Forward" 2.0 false)
      (`self.PlaySound` (`self.InCorrectSound`))
      (`UserWidget.BindToAnimationFinished` (`self.KeypadWidget`) _incorrect (`|CreateDelegate` :!event `AnimationFinished`))
      (if (`self.HasCompleteDialogue`)
        (if (not (`self.DialoguePlayed`))
          (bind _returnvalue_2 (`GameplayStatics.GetActorOfClass` "/Game/Blueprints/Dialogue_System/DialogueHolder.DialogueHolder_C"))
          (`/Game/Blueprints/Dialogue_System/DialogueHolder.AddDialogue` _returnvalue_2 (`self.DialogueArray_Failed`))
          (set `self.DialoguePlayed` true))))))

(fn `ComponentsToSave`
  (returns (Components :type "Array of ActorComponent Object Reference"))
  (return))

(fn `PlaySound`
  (params (InSound :type "SoundBase Object Reference"))
  (`GameplayStatics.PrimeSound` InSound)
  (`GameplayStatics.PlaySoundAtLocation` InSound (`SceneComponent.K2_GetComponentLocation` (`self.Keypad`)) (struct) 1.0 1.0 0.0 "/Game/Sound/ATN_Keypad.ATN_Keypad" null null))

(fn `UserConstructionScript`)