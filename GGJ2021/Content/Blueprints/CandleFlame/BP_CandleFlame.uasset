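; Candle flame Blueprint that flickers a point light and can be switched on or off.
; Tick feeds a random sub-second Delay into a FlipFlop that alternately plays and reverses the Flicker timeline, which lerps light intensity between MinIntensity and MaxIntensity.
; SetEnable toggles light and flame visibility and sets the static mesh's shadow casting to the opposite state.
; The construction script's SetEnable call is disconnected.
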(event `self.ReceiveBeginPlay`)

(event `self.ReceiveTick`
  (params (DeltaSeconds :type "Float (single-precision)"))
  (`KismetSystemLibrary.Delay` (`KismetMathLibrary.RandomFloatInRange` 0.1 0.8))
  (`/Engine/EditorBlueprintResources/StandardMacros.FlipFlop`
    (:`A`
      (bind (_direction _intensity) (`Timeline|Flicker` :!label _label)
        (:`Update`
          (`LightComponent.SetIntensity` (`self.PointLight`) (`KismetMathLibrary.Lerp` (`self.MinIntensity`) (`self.MaxIntensity`) _intensity)))))
    (:`B`
      (goto _label :!via `Reverse`))))

(fn `SetEnable`
  (params (Enabled :type Boolean))
  (bind _output_get (set `self.Enable` Enabled))
  (`SceneComponent.SetVisibility` (`self.PointLight`) _output_get false)
  (`SceneComponent.SetVisibility` (`self.CandleFlame`) _output_get false)
  (`PrimitiveComponent.SetCastShadow` (`self.StaticMesh`) (not _output_get)))

(fn `UserConstructionScript`)