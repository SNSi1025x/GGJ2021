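; BP_Weighted_AudioPlayer plays random sounds from its Sound array at irregular intervals, using configurable attenuation settings.
; Tick runs through a one-second Delay, then a weighted random roll decides whether to play.
; A DoOnce gate blocks new playback until the audio component's finished event resets it.
; ChangeSound is an empty event, and the InitialSound playback logic is disconnected.
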(event `self.ReceiveBeginPlay`
  (set `AudioComponent.AttenuationSettings` (`self.Attenuation Settings`) (`self.Audio`)))

(event `ChangeSound`)

(event `self.ReceiveTick`
  (params (DeltaSeconds :type "Float (single-precision)"))
  (bind _audio (`self.Audio`))
  (`KismetSystemLibrary.Delay` 1.0)
  (if (`KismetMathLibrary.RandomBoolWithWeight` (`self.Weight`))
    (`/Engine/EditorBlueprintResources/StandardMacros.DoOnce` false :!label _label
      (:`Completed`
        (`AudioComponent.SetSound` (`self.Audio`) (`|GetArrayItem` (`self.Sound`) (`KismetMathLibrary.RandomIntegerInRange` 0 (- (`KismetArrayLibrary.Array_Length` (`self.Sound`)) 1))))
        (`AudioComponent.Play` _audio 0.0)
        (add `AudioComponent.OnAudioFinished` _audio (delegate `Reset`))))))

(event `Reset`
  (goto _label :!via `Reset`))

(fn `UserConstructionScript`
  (set `AudioComponent.AttenuationSettings` (`self.Attenuation Settings`) (`self.Audio`)))