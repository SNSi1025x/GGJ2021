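; InteractOutline is a component that highlights a static mesh as interactable when overlapped.
; Overlap events turn custom depth rendering and a stencil value on and off, presumably feeding an outline post-process, and ticking is disabled at BeginPlay.
; Disconnected, never-run logic remains for spawning and toggling a Niagara effect on the mesh, with a height offset for a mesh named Sphere.
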(event `Overlap`
  (bind _staticmesh (`self.StaticMesh`))
  (`PrimitiveComponent.SetRenderCustomDepth` _staticmesh true)
  (`PrimitiveComponent.SetCustomDepthStencilValue` _staticmesh 2))

(event `EndOverlap`
  (bind _staticmesh (`self.StaticMesh`))
  (`PrimitiveComponent.SetRenderCustomDepth` _staticmesh false)
  (`PrimitiveComponent.SetCustomDepthStencilValue` _staticmesh 0))

(event `self.ReceiveBeginPlay`
  (`self.SetComponentTickEnabled` false))

(event `self.ReceiveTick`
  (params (DeltaSeconds :type "Float (single-precision)")))