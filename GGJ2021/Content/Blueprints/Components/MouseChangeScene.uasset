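; Actor component that makes its owner a clickable interactable for keypads, item pickups and magic-square puzzles.
; It binds cursor events on the owner's BoxComponent; clicks with the FirstPersonCharacter nearby open a widget chosen by InputType in UI-only input mode.
; Inspection types also add the component to the character's Inventory and disable the owner.
; Helper functions swap the FirstPersonHUD cursor texture; cursor-over is empty, while cursor-end sets Gold_Key and prints debug text.
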(event `self.ReceiveBeginPlay`
  (bind _returnvalue (`Actor.GetComponentByClass` (`self.GetOwner`) "/Script/Engine.BoxComponent"))
  (if (`KismetSystemLibrary.IsValid` _returnvalue)
    (bind _output_get (set `self.MyCollider` _returnvalue))
    (add `PrimitiveComponent.OnBeginCursorOver` _output_get (delegate `OnBeginCursorOver_Event_0`))
    (add `PrimitiveComponent.OnEndCursorOver` _output_get (delegate `OnEndCursorOver_Event_0`))
    (add `PrimitiveComponent.OnClicked` _output_get (delegate `OnClicked_Event_0`))))

(event `OnEndCursorOver_Event_0`
  (params (TouchedComponent :type "PrimitiveComponent Object Reference"))
  (`|ExecutionSequence`
    (:`then_0`
      (bind _outactors (`GameplayStatics.GetAllActorsOfClass` "/Game/FirstPersonBP/Blueprints/FirstPersonHUD.FirstPersonHUD_C"))
      (for _array_element _outactors
        (set `/Game/FirstPersonBP/Blueprints/FirstPersonHUD.MyTexture` "/Game/Materials/UI/Gold_Key.Gold_Key" _array_element)))
    (:`then_1`
      (cast `/Game/FirstPersonBP/Blueprints/FirstPersonCharacter` (`GameplayStatics.GetPlayerCharacter` 0)
        (:`then`
          (`KismetSystemLibrary.PrintString` "Mouse Change Scene Cast Success"))
        (:`CastFailed`
          (`KismetSystemLibrary.PrintString` "Mouse Change Scene Cast Failed"))))))

(event `OnClicked_Event_0`
  (params (TouchedComponent :type "PrimitiveComponent Object Reference") (ButtonPressed :type "Key Structure" :default "None"))
  (bind _returnvalue (`GameplayStatics.GetPlayerController` 0))
  (bind _returnvalue_2 (`GameplayStatics.GetPlayerController` 0))
  (bind _returnvalue_3 (`GameplayStatics.GetPlayerController` 0))
  (bind _outactors (`GameplayStatics.GetAllActorsOfClass` "/Game/FirstPersonBP/Blueprints/FirstPersonCharacter.FirstPersonCharacter_C"))
  (for _array_element _outactors
    (if (< (`Actor.GetDistanceTo` (`self.GetOwner`) _array_element) 500.0)
      (switch `int` (`self.InputType`)
        (:`1`
          (bind _returnvalue_4 (`|CreateWidget` "/Game/Blueprints/PuzzleBPs/Keypad/Keypad.Keypad_C" _returnvalue))
          (set `/Game/Blueprints/PuzzleBPs/Keypad/Keypad.KConnector` (`self.MConnector`) _returnvalue_4)
          (`UserWidget.AddToViewport` _returnvalue_4 0)
          (set `/Game/FirstPersonBP/Blueprints/FirstPersonCharacter.MouseHidden` false _array_element)
          (`WidgetBlueprintLibrary.SetInputMode_UIOnlyEx` _returnvalue _returnvalue_4)
          (set `PlayerController.bShowMouseCursor` true _returnvalue))
        (:`2`
          (bind _returnvalue_5 (`|CreateWidget` "/Game/Blueprints/Widgets/Inspection.Inspection_C" _returnvalue_2 :!label _label))
          (`Image.SetBrushFromTexture` (`/Game/Blueprints/Widgets/Inspection.MyImage` _returnvalue_5) (`self.MouseImage`) false)
          (`TextBlock.SetText` (`/Game/Blueprints/Widgets/Inspection.Name` _returnvalue_5) (`KismetTextLibrary.Conv_StringToText` (`self.Name`)))
          (`TextBlock.SetText` (`/Game/Blueprints/Widgets/Inspection.Description` _returnvalue_5) (`KismetTextLibrary.Conv_StringToText` (`self.Desc`)))
          (`/Game/Blueprints/Components/Inventory.AddItem` (`/Game/FirstPersonBP/Blueprints/FirstPersonCharacter.Inventory` _array_element) self)
          (`self.Disable`)
          (`UserWidget.AddToViewport` _returnvalue_5 0)
          (set `/Game/FirstPersonBP/Blueprints/FirstPersonCharacter.MouseHidden` false _array_element)
          (`WidgetBlueprintLibrary.SetInputMode_UIOnlyEx` _returnvalue_2 _returnvalue_5)
          (set `PlayerController.bShowMouseCursor` true _returnvalue_2))
        (:`3`
          (goto _label))
        (:`4`
          (if (not (`self.isPuzzleFinished`))
            (bind _returnvalue_6 (`|CreateWidget` "/Game/Blueprints/PuzzleBPs/MagicSquare/MagicSquare.MagicSquare_C" _returnvalue_3))
            (set `/Game/Blueprints/PuzzleBPs/MagicSquare/MagicSquare.IconSet` (`self.PuzzleSet`) _returnvalue_6)
            (set `/Game/Blueprints/PuzzleBPs/MagicSquare/MagicSquare.FirstPerson` _array_element _returnvalue_6)
            (bind _output_get (set `/Game/Blueprints/PuzzleBPs/MagicSquare/MagicSquare.StaticMeshActors` (`self.StaticMeshActors`) _returnvalue_6))
            (`|ExecutionSequence`
              (:`then_0`
                (`UserWidget.AddToViewport` _returnvalue_6 0)
                (set `/Game/FirstPersonBP/Blueprints/FirstPersonCharacter.MouseHidden` false _array_element)
                (`WidgetBlueprintLibrary.SetInputMode_UIOnlyEx` _returnvalue_3 _returnvalue_6)
                (set `PlayerController.bShowMouseCursor` true _returnvalue_3))
              (:`then_1`
                (for _ _output_get
                  _)))))))))

(event `OnBeginCursorOver_Event_0`
  (params (TouchedComponent :type "PrimitiveComponent Object Reference")))

(event `Disable`
  (bind _returnvalue (`self.GetOwner` self))
  (`Actor.SetActorHiddenInGame` _returnvalue true)
  (`Actor.SetActorEnableCollision` _returnvalue false)
  (`Actor.SetActorTickEnabled` _returnvalue false))

(event `self.ReceiveTick`
  (params (DeltaSeconds :type "Float (single-precision)")))

(fn `ChangeMouseHand`
  (`|ExecutionSequence`
    (:`then_0`
      (bind _outactors (`GameplayStatics.GetAllActorsOfClass` "/Game/FirstPersonBP/Blueprints/FirstPersonCharacter.FirstPersonCharacter_C"))
      (for _array_element _outactors
        (if (< (`Actor.GetDistanceTo` (`self.GetOwner`) _array_element) 500.0)
          (bind _outactors_2 (`GameplayStatics.GetAllActorsOfClass` "/Game/FirstPersonBP/Blueprints/FirstPersonHUD.FirstPersonHUD_C"))
          (for _array_element_2 _outactors_2
            (set `/Game/FirstPersonBP/Blueprints/FirstPersonHUD.MyTexture` "/Game/Materials/UI/Gold_Key2.Gold_Key2" _array_element_2)))))))

(fn `ChangeMouseNormal`
  (bind _outactors (`GameplayStatics.GetAllActorsOfClass` "/Game/FirstPersonBP/Blueprints/FirstPersonHUD.FirstPersonHUD_C"))
  (for _array_element _outactors
    (set `/Game/FirstPersonBP/Blueprints/FirstPersonHUD.MyTexture` "/Game/FirstPerson/Textures/FirstPersonCrosshair.FirstPersonCrosshair" _array_element)))