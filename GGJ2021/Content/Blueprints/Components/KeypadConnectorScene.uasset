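; Scene component that links its static mesh actor to a keypad and plays a swing-style yaw rotation when triggered.
; On BeginPlay it searches all static mesh actors for a MouseChangeScene whose RadioLink matches RecieverLink, storing a two-way reference.
; DoAction starts a Tick-driven, frame-rate-dependent rotation that adds one degree per frame up to 100, while setting a hardcoded relative location.
; The counter never resets.
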(event `self.ReceiveBeginPlay`
  (bind _outactors (`GameplayStatics.GetAllActorsOfClass` "/Script/Engine.StaticMeshActor"))
  (for _array_element _outactors
    (bind _returnvalue (`Actor.GetComponentByClass` _array_element "/Game/Blueprints/Components/MouseChangeScene.MouseChangeScene_C"))
    (if (`KismetSystemLibrary.IsValid` _returnvalue)
      (if (== (`self.RecieverLink`) (`/Game/Blueprints/Components/MouseChangeScene.RadioLink` _returnvalue))
        (set `self.Keypad` _returnvalue)
        (set `/Game/Blueprints/Components/MouseChangeScene.MConnector` self _returnvalue)))))

(event `self.ReceiveTick`
  (params (DeltaSeconds :type "Float (single-precision)"))
  (bind _time (`self.time`))
  (if (`self.isRunning`)
    (set `self.time` (+ _time 1.0))
    (bind _asstatic_mesh_actor (cast `StaticMeshActor` (`self.GetOwner`)))
    (`Actor.K2_SetActorRelativeRotation` _asstatic_mesh_actor (`KismetMathLibrary.MakeRotator` 0.0 0.0 (`self.time`)) false false)
    (`Actor.K2_SetActorRelativeLocation` _asstatic_mesh_actor (1009.939636 -189.543961 170.0) true false)
    (if (>= _time 100.0)
      (set `self.isRunning` false))))

(event `DoAction`
  (set `self.isRunning` true))