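; Trigger volume that retunes the player's sanity and flashlight behaviour when they enter its box.
; On overlap it casts to FirstPersonCharacter, then an enum selects whether to change sanity, flashlight or both.
; Helper functions copy the trigger's recharge and discharge values onto the character's in-light and out-of-light sanity rates and flashlight drain rate.
; Nothing restores the previous values on exit.
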(event `self.Box.OnComponentBeginOverlap`
  (params (OverlappedComponent :type "PrimitiveComponent Object Reference") (OtherActor :type "Actor Object Reference") (OtherComp :type "PrimitiveComponent Object Reference") (OtherBodyIndex :type Integer) (bFromSweep :type Boolean) (SweepResult :type "HitResult Structure (by ref)"))
  (bind _asfirst_person_character (cast `/Game/FirstPersonBP/Blueprints/FirstPersonCharacter` OtherActor))
  (set `self.FPC` _asfirst_person_character)
  (switch `/Game/Blueprints/Enums/Enum_SanityFlashlightTrigger` (`self.Enum`)
    (:`NewEnumerator0`
      (`self.ChangeSanity`))
    (:`NewEnumerator1`
      (`self.ChangeFlashlight`))
    (:`NewEnumerator2`
      (`self.ChangeSanity`)
      (`self.ChangeFlashlight`))))

(fn `ChangeFlashlight`
  (set `/Game/FirstPersonBP/Blueprints/FirstPersonCharacter.fFlashlightDischargeRate` (`self.FlashlightDischarge`) (`self.FPC`)))

(fn `ChangeSanity`
  (bind _fpc (`self.FPC`))
  (set `/Game/FirstPersonBP/Blueprints/FirstPersonCharacter.fSanityInLight` (`self.SanityRecharge`) _fpc)
  (set `/Game/FirstPersonBP/Blueprints/FirstPersonCharacter.fSanityOutLight` (`self.SanityDischarge`) _fpc))

(fn `UserConstructionScript`)