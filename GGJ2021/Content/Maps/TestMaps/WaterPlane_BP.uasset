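; WaterPlane_BP is a test-map water surface that switches scene fog between above-water and underwater looks.
; Each begin overlap with the FirstPersonCharacter flips IsInWater, so crossing the plane toggles the state; end overlap does nothing.
; Entering applies WaterFogColor and denser fog to the referenced Fog component; the next crossing applies FogOriginalColor and a lower, hardcoded density.
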(event `self.ReceiveActorBeginOverlap`
  (params (OtherActor :type "Actor Object Reference"))
  (bind _component (`ExponentialHeightFog.Component` (`self.Fog`)))
  (cast `/Game/FirstPersonBP/Blueprints/FirstPersonCharacter` OtherActor)
  (if (`self.IsInWater`)
    (`ExponentialHeightFogComponent.SetFogInscatteringColor` (`ExponentialHeightFog.Component` (`self.Fog`)) (`self.FogOriginalColor`))
    (`ExponentialHeightFogComponent.SetFogInscatteringColor` _component (`self.FogOriginalColor`))
    (`ExponentialHeightFogComponent.SetFogDensity` _component 0.5)
    (set `self.IsInWater` false)
    (else
      (`ExponentialHeightFogComponent.SetFogInscatteringColor` _component (`self.WaterFogColor`))
      (`ExponentialHeightFogComponent.SetFogDensity` _component 1.5)
      (set `self.IsInWater` true))))

(event `self.ReceiveActorEndOverlap`
  (params (OtherActor :type "Actor Object Reference")))

(fn `UserConstructionScript`)