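; Interactable lamp switch that tilts the lamp and removes a separate HiddenPlane actor when used.
; Overlapping the box trigger enables player input on this actor, and leaving it disables input.
; Pressing Interact plays the LampTilt timeline, which drives the lamp's relative roll.
; The timeline's update also destroys the trigger and HiddenPlane, removing the overlap zone after use.
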(event `self.BoxTrigger.OnComponentBeginOverlap`
  (params (OverlappedComponent :type "PrimitiveComponent Object Reference") (OtherActor :type "Actor Object Reference") (OtherComp :type "PrimitiveComponent Object Reference") (OtherBodyIndex :type Integer) (bFromSweep :type Boolean) (SweepResult :type "HitResult Structure (by ref)"))
  (`self.EnableInput` (`GameplayStatics.GetPlayerController` 0)))

(event `self.BoxTrigger.OnComponentEndOverlap`
  (params (OverlappedComponent :type "PrimitiveComponent Object Reference") (OtherActor :type "Actor Object Reference") (OtherComp :type "PrimitiveComponent Object Reference") (OtherBodyIndex :type Integer))
  (`self.DisableInput` (`GameplayStatics.GetPlayerController` 0)))

(event `InputAction|Interact`
  (params (Key :type "Key Structure"))
  (:`Pressed`
    (bind (_direction _lamptilt) (`Timeline|LampTilt`)
      (:`Update`
        (`SceneComponent.K2_SetRelativeRotation` (`self.Lamp`) (`KismetMathLibrary.MakeRotator` _lamptilt) false false)
        (`ActorComponent.K2_DestroyComponent` (`self.BoxTrigger`))
        (`self.K2_DestroyActor` (`self.HiddenPlane`))))))

(fn `UserConstructionScript`)