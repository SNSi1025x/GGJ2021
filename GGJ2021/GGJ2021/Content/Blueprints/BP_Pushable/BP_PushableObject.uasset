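; Pushable cube that the player can shove, and that returns to its start position when it leaves its BP_BlockBounds area.
; Overlapping either axis trigger shows an interact outline and enables cube physics unless Tripped, and leaving disables both.
; A delayed Tick checks bounds; when out, a timeline lerps the cube home.
; A DoOnce, reset when the lerp finishes, applies the sanity and flashlight charge changes to the player.
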(event `self.ReceiveBeginPlay`
  (`self.SetActorTickEnabled` true)
  (set `self.StartLocation` (`SceneComponent.K2_GetComponentLocation` (`self.Cube`))))

(event `self.ReceiveTick`
  (params (DeltaSeconds :type "Float (single-precision)"))
  (`KismetSystemLibrary.Delay` 1.0)
  (`self.CheckInBounds`)
  (if (not (`self.inBounds`))
    (bind (_direction _lerp) (`Timeline|Lerp 0 -1` :!via `PlayFromStart`)
      (:`Update`
        (`SceneComponent.K2_SetWorldLocation` (`self.Cube`) (`KismetMathLibrary.VLerp` (`SceneComponent.K2_GetComponentLocation` (`self.Cube`)) (`self.StartLocation`) _lerp) false false)
        (`/Engine/EditorBlueprintResources/StandardMacros.DoOnce` false :!label _label
          (:`Completed`
            (bind _asfirst_person_character (cast `/Game/FirstPersonBP/Blueprints/FirstPersonCharacter` (`GameplayStatics.GetPlayerCharacter` 0)))
            (set `self.FPC` _asfirst_person_character)
            (`self.IncreaseDecreaseSanity` (`self.SanityDrop`))
            (`self.IncreaseDecreaseCharge` (`self.ChargeDrop`)))))
      (:`Finished`
        (goto _label :!via `Reset`)))))

(event `self.XAxis.OnComponentBeginOverlap`
  (params (OverlappedComponent :type "PrimitiveComponent Object Reference") (OtherActor :type "Actor Object Reference") (OtherComp :type "PrimitiveComponent Object Reference") (OtherBodyIndex :type Integer) (bFromSweep :type Boolean) (SweepResult :type "HitResult Structure (by ref)"))
  (bind _interactoutline (`self.InteractOutline`))
  (if (not (`self.Tripped`))
    (cast `/Game/FirstPersonBP/Blueprints/FirstPersonCharacter` OtherActor)
    (set `/Game/Blueprints/Components/InteractOutline.StaticMesh` (`self.Cube`) _interactoutline)
    (`/Game/Blueprints/Components/InteractOutline.Overlap` _interactoutline)
    (`self.SetActorTickEnabled` true)
    (`PrimitiveComponent.SetSimulatePhysics` (`self.Cube`) true)
    (`KismetSystemLibrary.PrintString` "XAxisBegin")))

(event `self.XAxis.OnComponentEndOverlap`
  (params (OverlappedComponent :type "PrimitiveComponent Object Reference") (OtherActor :type "Actor Object Reference") (OtherComp :type "PrimitiveComponent Object Reference") (OtherBodyIndex :type Integer))
  (cast `/Game/FirstPersonBP/Blueprints/FirstPersonCharacter` OtherActor)
  (`/Game/Blueprints/Components/InteractOutline.EndOverlap` (`self.InteractOutline`))
  (`self.SetActorTickEnabled` true)
  (`PrimitiveComponent.SetSimulatePhysics` (`self.Cube`) false)
  (`KismetSystemLibrary.PrintString` "XAxisEnd"))

(event `self.YAxis.OnComponentBeginOverlap`
  (params (OverlappedComponent :type "PrimitiveComponent Object Reference") (OtherActor :type "Actor Object Reference") (OtherComp :type "PrimitiveComponent Object Reference") (OtherBodyIndex :type Integer) (bFromSweep :type Boolean) (SweepResult :type "HitResult Structure (by ref)"))
  (bind _interactoutline (`self.InteractOutline`))
  (if (not (`self.Tripped`))
    (cast `/Game/FirstPersonBP/Blueprints/FirstPersonCharacter` OtherActor)
    (set `/Game/Blueprints/Components/InteractOutline.StaticMesh` (`self.Cube`) _interactoutline)
    (`/Game/Blueprints/Components/InteractOutline.Overlap` _interactoutline)
    (`self.SetActorTickEnabled` true)
    (`PrimitiveComponent.SetSimulatePhysics` (`self.Cube`) true)
    (`KismetSystemLibrary.PrintString` "YAxisBegin")))

(event `self.YAxis.OnComponentEndOverlap`
  (params (OverlappedComponent :type "PrimitiveComponent Object Reference") (OtherActor :type "Actor Object Reference") (OtherComp :type "PrimitiveComponent Object Reference") (OtherBodyIndex :type Integer))
  (cast `/Game/FirstPersonBP/Blueprints/FirstPersonCharacter` OtherActor)
  (`/Game/Blueprints/Components/InteractOutline.EndOverlap` (`self.InteractOutline`))
  (`self.SetActorTickEnabled` true)
  (`PrimitiveComponent.SetSimulatePhysics` (`self.Cube`) false)
  (`KismetSystemLibrary.PrintString` "YAxisEnd"))

(fn `CheckInBounds`
  (bind _overlappingactors (`self.GetOverlappingActors` "/Game/Blueprints/BP_Pushable/BP_BlockBounds.BP_BlockBounds_C"))
  (if (`KismetSystemLibrary.IsValid` (`self.Bounds`))
    (`|ExecutionSequence`
      (:`then_0`
        (set `self.inBounds` (`KismetArrayLibrary.Array_Contains` _overlappingactors (stale _array_element))))
      (:`then_1`
        (for _array_element _overlappingactors
          _)))))

(fn `IncreaseDecreaseCharge`
  (params (Charge :type "Float (double-precision)"))
  (bind _fpc (`self.FPC`))
  (set `/Game/FirstPersonBP/Blueprints/FirstPersonCharacter.fFlashlighCurrentCharge` (`KismetMathLibrary.FClamp` (+ (`/Game/FirstPersonBP/Blueprints/FirstPersonCharacter.fFlashlighCurrentCharge` _fpc) Charge) 0.0 (`/Game/FirstPersonBP/Blueprints/FirstPersonCharacter.fFlashlightMaxCharge` _fpc)) (`self.FPC`)))

(fn `IncreaseDecreaseSanity`
  (params (Sanity :type "Float (double-precision)"))
  (bind _fpc (`self.FPC`))
  (set `/Game/FirstPersonBP/Blueprints/FirstPersonCharacter.fCurrentSanity` (`KismetMathLibrary.FClamp` (+ (`/Game/FirstPersonBP/Blueprints/FirstPersonCharacter.fCurrentSanity` _fpc) Sanity) 0.0 (`/Game/FirstPersonBP/Blueprints/FirstPersonCharacter.fMaxSanity` _fpc)) (`self.FPC`)))

(fn `UserConstructionScript`)