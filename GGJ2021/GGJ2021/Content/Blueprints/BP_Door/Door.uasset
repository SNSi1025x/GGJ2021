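; Interactable door that swings open and closed on a timeline-driven yaw lerp and can be locked.
; Trigger overlap shows an outline and HUD prompt, enables input and opens a gate so Interact toggles the door when unlocked.
; Unlock clears the lock, Solved unlocks and opens a closed door, and LeverToggle closes an open one.
; Key possession is set externally; interacting with an unlocked door while holding it marks the key used.
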(event `/Game/Blueprints/Interfaces/I_Unlock.Unlock`
  (set `self.isLocked` false))

(event `/Game/Blueprints/Interfaces/I_Puzzle.Solved`
  (params (Block :type "/Game/Blueprints/BP_Pushable/BP_PushableObject Object Reference"))
  (if (`self.isClosed`)
    (set `self.isLocked` false)
    (if (== (`self.isClosed`) true) :!label _label
      (set `self.isClosed` false)
      (bind (_direction _door) (`Timeline|Door Timeline` :!via `ReverseFromEnd` :!label _label_2)
        (:`Update`
          (`SceneComponent.K2_SetRelativeRotation` (`self.InteriorDoor_InteriorDoor`) (`KismetMathLibrary.MakeRotator` 0.0 0.0 (`KismetMathLibrary.Lerp` (`self.DoorOpenAngle`) (`self.DoorCloseAngle`) _door)) false false)))
      (else
        (set `self.isClosed` true)
        (goto _label_2 :!via `PlayFromStart`)))))

(event `self.ReceiveTick`
  (params (DeltaSeconds :type "Float (single-precision)")))

(event `/Game/Blueprints/Interfaces/I_Lever.LeverToggle`
  (params (Lever :type "/Game/Blueprints/PuzzleBPs/LeverPuzzle/BP_LeverPuzzle Object Reference"))
  (if (not (`self.isClosed`))
    (goto _label)))

(event `InputAction|Interact`
  (params (Key :type "Key Structure"))
  (:`Pressed`
    (if (not (`self.isLocked`))
      (`/Engine/EditorBlueprintResources/StandardMacros.Gate` true :!label _label_3
        (:`Exit`
          (`|ExecutionSequence`
            (:`then_0`
              (goto _label))
            (:`then_1`
              (if (`self.hasKey`)
                (set `self.keyUsed` true)))))))))

(event `self.InteractTrigger.OnComponentBeginOverlap`
  (params (OverlappedComponent :type "PrimitiveComponent Object Reference") (OtherActor :type "Actor Object Reference") (OtherComp :type "PrimitiveComponent Object Reference") (OtherBodyIndex :type Integer) (bFromSweep :type Boolean) (SweepResult :type "HitResult Structure (by ref)"))
  (bind _interactoutline (`self.InteractOutline`))
  (bind _hud (`/Game/FirstPersonBP/Blueprints/FirstPersonCharacter.HUD` (`self.FPC`)))
  (bind _asfirst_person_character (cast `/Game/FirstPersonBP/Blueprints/FirstPersonCharacter` OtherActor))
  (set `self.FPC` _asfirst_person_character)
  (set `/Game/Blueprints/Components/InteractOutline.StaticMesh` (`self.InteriorDoor_InteriorDoor`) _interactoutline)
  (`/Game/Blueprints/Components/InteractOutline.Overlap` _interactoutline)
  (if (`self.isLocked`)
    (set `/Game/Blueprints/Widgets/HUD.PopUpText` "Door is locked" _hud)
    (elif (`self.isClosed`)
      (set `/Game/Blueprints/Widgets/HUD.PopUpText` "Press E To Open" _hud)
      (else
        (set `/Game/Blueprints/Widgets/HUD.PopUpText` "Press E To Close" _hud))))
  (`self.EnableInput` (`GameplayStatics.GetPlayerController` 0))
  (goto _label_3 :!via `Open`))

(event `self.InteractTrigger.OnComponentEndOverlap`
  (params (OverlappedComponent :type "PrimitiveComponent Object Reference") (OtherActor :type "Actor Object Reference") (OtherComp :type "PrimitiveComponent Object Reference") (OtherBodyIndex :type Integer))
  (cast `/Game/FirstPersonBP/Blueprints/FirstPersonCharacter` OtherActor)
  (`/Game/Blueprints/Components/InteractOutline.EndOverlap` (`self.InteractOutline`))
  (set `/Game/Blueprints/Widgets/HUD.PopUpText` "" (`/Game/FirstPersonBP/Blueprints/FirstPersonCharacter.HUD` (`self.FPC`)))
  (`self.DisableInput` (`GameplayStatics.GetPlayerController` 0))
  (goto _label_3 :!via `Close`))

(fn `PlayerHasKey`
  (params (PlayHasKey :type Boolean))
  (set `self.hasKey` PlayHasKey)
  (return))

(fn `PlayerUsedKey`
  (returns (usedKey :type Boolean))
  (return (`self.keyUsed`)))

(fn `UserConstructionScript`)