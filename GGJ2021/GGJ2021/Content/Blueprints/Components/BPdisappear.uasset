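; Actor component that makes its owning object disappear or reappear based on the player's sanity, changing it only while the object is off-screen.
; Tick, throttled by a short Delay, projects the owner's location to screen space and tests it against the padded viewport bounds.
; When outside, it compares FirstPersonCharacter's current sanity to a threshold, hiding the root component and its children at or below it and showing them otherwise.
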(event `self.ReceiveTick`
  (params (DeltaSeconds :type "Float (single-precision)"))
  (bind (_returnvalue_x _returnvalue_y) (`KismetMathLibrary.BreakVector2D` (`WidgetLayoutLibrary.GetViewportSize`)))
  (bind _rootcomponent (`Actor.RootComponent` (`self.GetOwner`)))
  (bind _screenlocation (`PlayerController.ProjectWorldLocationToScreen` (`GameplayStatics.GetPlayerController` 0) (`Actor.K2_GetActorLocation` (`self.GetOwner`)) false))
  ;[1 1 1] Check players sanity against the sanity threshold and then set visibility.
  (`KismetSystemLibrary.Delay` 0.25)
  (bind _asfirst_person_character (cast `/Game/FirstPersonBP/Blueprints/FirstPersonCharacter` (`GameplayStatics.GetPlayerCharacter` 0)))
  (if (and (`KismetMathLibrary.InRange_FloatFloat` (`KismetMathLibrary.BreakVector2D` _screenlocation) -500.0 (+ _returnvalue_x 500.0)) (`KismetMathLibrary.InRange_FloatFloat` (`.Y` (`KismetMathLibrary.BreakVector2D` _screenlocation)) -500.0 (+ _returnvalue_y 500.0)))
    _
    (elif (<= (`/Game/FirstPersonBP/Blueprints/FirstPersonCharacter.fCurrentSanity` _asfirst_person_character) (`self.fSanityThreshold`))
      (`SceneComponent.SetVisibility` _rootcomponent false true)
      (else
        (`SceneComponent.SetVisibility` _rootcomponent true true)))))