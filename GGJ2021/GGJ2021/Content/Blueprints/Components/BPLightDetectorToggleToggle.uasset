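; An actor component for a Light that switches its linked light detectors on and off with the light.
; Every tick it casts its owner to Light and reads whether the light component is visible.
; It then loops over the LightDetectors array, enabling query-only collision on each LightDetection trigger while the light is visible and disabling collision otherwise.
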(event `self.ReceiveBeginPlay`)

(event `self.ReceiveTick`
  (params (DeltaSeconds :type "Float (single-precision)"))
  ;[1 1 1] Gets the owner of this component, Gets all actors of the array and then sets collision based on owners visibility
  (bind _aslight (cast `Light` (`self.GetOwner`)))
  (set `self.bLightOn` (`SceneComponent.IsVisible` (`Light.LightComponent` _aslight)))
  (for _array_element (`self.LightDetectors`)
    (bind _aslight_detection (cast `/Game/Blueprints/PropBlueprints/LightDetection` _array_element))
    (if (`self.bLightOn`)
      (bind _trigger (`/Game/Blueprints/PropBlueprints/LightDetection.Trigger` _aslight_detection))
      (`PrimitiveComponent.SetCollisionEnabled` _trigger "QueryOnly")
      (else
        (`PrimitiveComponent.SetCollisionEnabled` _trigger "NoCollision")))))